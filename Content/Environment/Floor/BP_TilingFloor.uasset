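; BP_TilingFloor is a floor actor that tints its material to match a season.
; The construction script creates a dynamic material on the Floor component and applies ForceSeason immediately when one is set.
; When ForceSeason holds its sentinel enum value, BeginPlay instead picks a random key from the SeasonDisplays map.
; UpdateSeasonDisplay looks up that season's entry and writes its hue shift, desaturation and darken values to the material.
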(event EventBeginPlay
  (if (Utilities|Enum|Equal(Enum) (Variables|Default|GetForceSeason) "NewEnumerator5")
    (bind _keys (Utilities|Map|Keys (Variables|Default|GetSeasonDisplays)))
    (Variables|Default|SetSeason (.OutItem (Utilities|Array|Random _keys)))
    (CallFunction|UpdateSeasonDisplay)))

(fn ConstructionScript
  (bind _floor (Variables|Default|GetFloor))
  (bind _forceseason (Variables|Default|GetForceSeason))
  (bind _returnvalue (Rendering|Material|CreateDynamicMaterialInstance _floor 0 (Rendering|Material|GetMaterial _floor 0) "None" :!class /Script/Engine.PrimitiveComponent))
  (Variables|Default|SetDynamicMaterial _returnvalue)
  (if (Utilities|Enum|NotEqual(Enum) _forceseason "NewEnumerator5")
    (Variables|Default|SetSeason _forceseason)
    (CallFunction|UpdateSeasonDisplay)))

(fn UpdateSeasonDisplay
  (bind _season (Variables|Default|GetSeason))
  (bind _seasondisplays (Variables|Default|GetSeasonDisplays))
  (bind _dynamicmaterial (Variables|Default|GetDynamicMaterial))
  (bind (_value _returnvalue) (Utilities|Map|Find _seasondisplays _season))
  (bind (_hueshift _desaturation _darken) (Utilities|Struct|BreakS_SeasonDisplay _value))
  (if _returnvalue
    (Rendering|Material|SetScalarParameterValue _dynamicmaterial "HueShift" _hueshift :!class /Script/Engine.MaterialInstanceDynamic)
    (Rendering|Material|SetScalarParameterValue _dynamicmaterial "Desaturation" _desaturation :!class /Script/Engine.MaterialInstanceDynamic)
    (Rendering|Material|SetScalarParameterValue _dynamicmaterial "Darken" _darken :!class /Script/Engine.MaterialInstanceDynamic)
    (return)
    (else
      (return))))