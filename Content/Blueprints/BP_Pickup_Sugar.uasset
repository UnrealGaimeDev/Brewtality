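; Sugar cube pickup that grants experience to the BP_Teapot that overlaps it.
; A Quantity setting picks the material, the randomized scale and the experience amount, and the mesh gets a random rotation at BeginPlay.
; On first overlap, a timeline animates the mesh between its original spot and the player's live location with a Z offset and scaling.
; When the timeline finishes, it awards the experience and destroys the actor.
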(event Custom|Pickup
  (params (Player :type BP%20Teapot%20Object%20Reference))
  (if (not (Variables|Default|GetPickedUp?))
    (Variables|Default|SetPickedUp? true)
    (Variables|Default|SetPlayer Player)
    (Variables|Default|SetOriginalLocation (Transformation|GetWorldLocation (Variables|Character|GetMesh)))
    (Variables|Default|SetOriginalScale (Variables|/Script/Engine.SceneComponent|GetRelativeScale3D (Variables|Character|GetMesh)))
    (bind (_direction _distance _zoffset _scale) (Timeline|AnimationTimeline PlayFromStart)
      (:Update
        (Transformation|SetWorldLocation (Variables|Character|GetMesh) (+ (Math|Vector|Lerp(Vector) (Transformation|GetActorLocation (Variables|Default|GetPlayer)) (Variables|Default|GetOriginalLocation) _distance) (Math|Vector|MakeVector 0.0 0.0 (Math|Float|Lerp 0.0 (Variables|Default|GetMaxZOffset) _zoffset))) false false)
        (Transformation|SetRelativeScale3D (Variables|Character|GetMesh) (* (Variables|Default|GetOriginalScale) _scale)))
      (:Finished
        (Default|AddExperience (Variables|Default|GetPlayer) (.Value (Utilities|Map|Find (Variables|Default|GetExperiencePerQuantity) (Variables|Default|GetQuantity))))
        (Actor|DestroyActor)))))

(event EventBeginPlay
  (|CallParentFunction)
  (Transformation|SetRelativeRotation (Variables|Character|GetMesh) (Math|Random|RandomRotator false) false false))

(event Collision|EventActorBeginOverlap
  (params (OtherActor :type Actor%20Object%20Reference))
  (|CallParentFunction OtherActor) ; This node is disabled and will not be called.\nDrag off pins to build functionality.
)

(event EventTick
  (params (DeltaSeconds :type Float%20%28single-precision%29))
  (|CallParentFunction DeltaSeconds) ; This node is disabled and will not be called.\nDrag off pins to build functionality.
)

(event EventOnOverlap
  (params (Actor :type Actor%20Object%20Reference))
  (if (not (Variables|Default|GetPickedUp?))
    (|CallParentFunction Actor)
    (bind _asbp_teapot (Utilities|Casting|CastToBP_Teapot Actor))
    (CallFunction|Pickup _asbp_teapot)))

(fn ConstructionScript
  (bind _scaleperquantity (Variables|Default|GetScalePerQuantity))
  (bind _quantity (Variables|Default|GetQuantity))
  (bind _value (Utilities|Map|Find _scaleperquantity _quantity))
  (|CallParentFunction)
  (Transformation|SetActorRelativeScale3D (Math|Conversions|ToVector(Float) (Math|Random|RandomFloatinRange (- _value (Variables|Default|GetScaleVariation)) (+ _value (Variables|Default|GetScaleVariation)))))
  (Rendering|Material|SetMaterial (Variables|Character|GetMesh) 0 (Utilities|Select :Index (Variables|Default|GetQuantity) :NewEnumerator3 0 :NewEnumerator0 "/Game/ToonShader/MI_SugarCube_Small.MI_SugarCube_Small" :NewEnumerator1 "/Game/ToonShader/MI_SugarCube_Medium.MI_SugarCube_Medium" :NewEnumerator2 "/Game/ToonShader/MI_SugarCube_Large.MI_SugarCube_Large")))