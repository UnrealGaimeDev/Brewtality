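; BP_Damage_AoE is an area-of-effect damage actor that damages damageable actors inside a hidden collision sphere.
; TriggerAoE stores normal and critical damage info, then UpdateRadius resizes the sphere and runs DamageEnemies on its overlaps.
; Each I_Damageable target that accepts the damage is hit only once, tracked in DamagedActors, with its own random crit roll.
; EndAoE destroys the actor.
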(event Custom|TriggerAoE
  (params (Damage :type S%20Damage%20Structure) (Radius :type Float%20%28single-precision%29) (CritPercentage :type Float%20%28double-precision%29) (CritMultiplier :type Float%20%28double-precision%29))
  (bind _output_get (Variables|Default|SetDamageInfo Damage))
  (Variables|Default|SetCritDamageInfo (Utilities|Struct|MakeS_Damage (* (.Amount (Utilities|Struct|BreakS_Damage _output_get)) CritMultiplier) (.SourceType (Utilities|Struct|BreakS_Damage _output_get)) (.SourceActor (Utilities|Struct|BreakS_Damage _output_get)) (.Knockback (Utilities|Struct|BreakS_Damage _output_get)) true (.Type (Utilities|Struct|BreakS_Damage _output_get))))
  (Variables|Default|SetCritChance CritPercentage)
  (CallFunction|UpdateRadius Radius))

(event Custom|EndAoE
  (Actor|DestroyActor))

(fn ConstructionScript
  (Development|SetHiddeninGame (Variables|Default|GetCollisionSphere) true false))

(fn DamageEnemies
  (for _array_element (Collision|GetOverlappingActors (Variables|Default|GetCollisionSphere) 0 :!class /Script/Engine.PrimitiveComponent)
    (Utilities|IsValid _array_element
      (:Is%20Valid
        (if (Utilities|DoesObjectImplementInterface _array_element "/Game/Blueprints/Interfaces/I_Damageable.I_Damageable_C")
          (if (not (Utilities|Set|Contains (Variables|Default|GetDamagedActors) _array_element))
            (bind _out_ (Class|IDamageable|CanReceiveDamage?(Message) _array_element (Variables|Default|GetDamageInfo)))
            (if _out_
              (Utilities|Set|Add (Variables|Default|GetDamagedActors) _array_element)
              (bind _out (CallFunction|RandomBoolfromChance (Variables|Default|GetCritChance)))
              (Class|IDamageable|ReceiveDamage(Message) _array_element (select _out (Variables|Default|GetCritDamageInfo) (Variables|Default|GetDamageInfo))))))))))

(fn UpdateRadius
  (params (NewRadius :type Float%20%28single-precision%29))
  (bind _output_get (Variables|Default|SetRadius NewRadius))
  (Components|Sphere|SetSphereRadius (Variables|Default|GetCollisionSphere) _output_get true)
  (CallFunction|DamageEnemies))