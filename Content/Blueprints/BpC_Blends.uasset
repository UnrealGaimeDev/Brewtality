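; Player component that tracks crafting blends from DT_Blends and activates each one once its recipe's ingredient amounts are met.
; When an ingredient is added, it checks remaining blends whose recipes use that ingredient against the player's Ingredients component.
; Activation moves the blend from remaining to activated, unlocks its listed ingredients, prints a message and adds a display to the main widget.
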(event Custom|Initialize
  (params (Player :type BP%20Teapot%20Object%20Reference))
  (Variables|Default|SetPlayerRef Player)
  (bind _outrownames (DataTable|GetDataTableRowNames "/Game/Blueprints/DataTables/DT_Blends.DT_Blends"))
  (Variables|Default|SetRemainingBlends _outrownames))

(event Custom|OnBlendActivated
  (params (Blend :type Name))
  (Development|PrintString (Utilities|String|Append "Activated blend: " (Utilities|String|ToString(Name) Blend)))
  (Default|AddBlendDisplay (Variables|/Game/Blueprints/BP_TeapotController.BP_TeapotController_C|GetMainWidgetRef (Variables|/Game/Blueprints/BP_Teapot.BP_Teapot_C|GetControllerRef (Variables|Default|GetPlayerRef))) Blend))

(event Custom|OnIngredientAdded
  (params (Ingredient :type Name))
  (bind _blendstoactivate (CallFunction|HasCompletedRecipes? Ingredient false))
  (for _array_element _blendstoactivate
    (CallFunction|ActivateBlend _array_element)))

(fn IsBlendActive?
  (params (Blend :type Name))
  (return (Utilities|Array|ContainsItem (Variables|Default|GetActivatedBlends) Blend)))

(fn ActivateBlend
  (params (Blend :type Name))
  (LocalVariables|SetlocalBlend Blend)
  (if (CallFunction|IsBlendActive? (LocalVariables|GetlocalBlend))
    (return)
    (else
      (Utilities|Array|RemoveItem (Variables|Default|GetRemainingBlends) (LocalVariables|GetlocalBlend))
      (Utilities|Array|Add (Variables|Default|GetActivatedBlends) (LocalVariables|GetlocalBlend))
      (bind _info (CallFunction|GetBlendInfo (LocalVariables|GetlocalBlend)))
      (for _array_element (Utilities|Struct|BreakS_TeaBlend _info)
        (Default|UnlockIngredient (Variables|/Game/Blueprints/BP_Teapot.BP_Teapot_C|GetIngredients (Variables|Default|GetPlayerRef)) _array_element))
      (CallFunction|OnBlendActivated (LocalVariables|GetlocalBlend))
      (return))))

(fn GetBlendInfo
  (params (Blend :type Name))
  (bind _returnvalue (Utilities|GetDataTableRow "/Game/Blueprints/DataTables/DT_Blends.DT_Blends" Blend)
    (:then
      (return _returnvalue))
    (:RowNotFound
      (return ""))))

(fn HasCompletedRecipes?
  (params (AddedIngredient :type Name) (CheckAll? :type Boolean))
  (LocalVariables|SetlocalAddedIngredient AddedIngredient)
  (for _array_element (Variables|Default|GetRemainingBlends)
    (LocalVariables|SetlocalBlend _array_element)
    (bind _info (CallFunction|GetBlendInfo (LocalVariables|GetlocalBlend)))
    (if (or (.ReturnValue (Utilities|Map|Find (Utilities|Struct|BreakS_TeaBlend _info) (LocalVariables|GetlocalAddedIngredient))) CheckAll?)
      (LocalVariables|SetlocalRecipeComplete true)
      (bind _keys (Utilities|Map|Keys (Utilities|Struct|BreakS_TeaBlend _info)))
      (bind _array_element_2 (Utilities|Array|ForEachLoopwithBreak _keys :!label _label)
        (:LoopBody
          (bind _amount (Default|GetIngredient (Variables|/Game/Blueprints/BP_Teapot.BP_Teapot_C|GetIngredients (Variables|Default|GetPlayerRef)) _array_element_2))
          (if (not (>= _amount (.Value (Utilities|Map|Find (Utilities|Struct|BreakS_TeaBlend _info) _array_element_2))))
            (LocalVariables|SetlocalRecipeComplete false)
            (goto _label Break)))
        (:Completed
          (if (LocalVariables|GetlocalRecipeComplete)
            (Utilities|Array|Add (LocalVariables|GetlocalCompletedBlends) (LocalVariables|GetlocalBlend)))))))
  (return (LocalVariables|GetlocalCompletedBlends)))