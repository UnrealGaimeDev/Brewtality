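; Sugar pickup that is tossed out on spawn and becomes collectible after its first hit.
; BeginPlay disables the PickupRange collision, runs the parent logic, then launches the physics mesh with a random horizontal and upward impulse drawn from velocity ranges.
; On the mesh's hit event, gravity and physics stop, the mesh ignores all collision channels, and PickupRange collision is re-enabled, preventing pickup mid-flight.
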(event OnComponentHit(Mesh)
  (params (HitComponent :type Primitive%20Component%20Object%20Reference) (OtherActor :type Actor%20Object%20Reference) (OtherComp :type Primitive%20Component%20Object%20Reference) (NormalImpulse :type Vector :default "0, 0, 0") (Hit :type Hit%20Result%20Structure%20%28by%20ref%29))
  (bind _mesh (Variables|Character|GetMesh))
  (Physics|SetEnableGravity _mesh false)
  (Physics|SetSimulatePhysics _mesh false)
  (Collision|SetCollisionResponsetoAllChannels _mesh "ECR_Ignore")
  (Collision|SetCollisionEnabled (Variables|Default|GetPickupRange) "QueryAndPhysics"))

(event EventBeginPlay
  (bind _horizontalvelocity (Variables|Default|GetHorizontalVelocity))
  (bind _upvelocity (Variables|Default|GetUpVelocity))
  (bind (_min _max) (Utilities|Struct|BreakS_Bounds _upvelocity))
  (bind (_min_2 _max_2) (Utilities|Struct|BreakS_Bounds _horizontalvelocity))
  (Collision|SetCollisionEnabled (Variables|Default|GetPickupRange) "NoCollision")
  (|CallParentFunction)
  (Physics|AddImpulse (Variables|Character|GetMesh) (+ (* (Math|Vector|Normalize (Math|Vector|MakeVector (Math|Random|RandomFloatinRange -1.0 1.0) (Math|Random|RandomFloatinRange -1.0 1.0) 0.0)) (Math|Random|RandomFloatinRange _min_2 _max_2)) (* (Math|Vector|VectorUp) (Math|Random|RandomFloatinRange _min _max))) "None" false))

(event Collision|EventActorBeginOverlap
  (params (OtherActor :type Actor%20Object%20Reference))
  (|CallParentFunction OtherActor) ; This node is disabled and will not be called.\nDrag off pins to build functionality.
)

(event EventTick
  (params (DeltaSeconds :type Float%20%28single-precision%29))
  (|CallParentFunction DeltaSeconds) ; This node is disabled and will not be called.\nDrag off pins to build functionality.
)

(fn ConstructionScript
  (|CallParentFunction))