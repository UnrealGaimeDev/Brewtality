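; BP_CirclePoint is an activation point that a boiling BP_Teapot triggers by entering its radius.
; The construction script sizes the Radius sphere from ActivationRadius.
; On overlap with a boiling teapot, it sets an Activated flag and adds an activated point to that teapot's PlayerStatistics, ignoring repeats.
; Deactivate only clears the flag, allowing the point to be activated again.
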(event OnComponentBeginOverlap(Radius)
  (params (OverlappedComponent :type Primitive%20Component%20Object%20Reference) (OtherActor :type Actor%20Object%20Reference) (OtherComp :type Primitive%20Component%20Object%20Reference) (OtherBodyIndex :type Integer) (bFromSweep :type Boolean) (SweepResult :type Hit%20Result%20Structure%20%28by%20ref%29))
  (bind _asbp_teapot (Utilities|Casting|CastToBP_Teapot OtherActor))
  (if (Variables|/Game/Blueprints/BP_Teapot.BP_Teapot_C|GetBoiling? _asbp_teapot)
    (CallFunction|Activate _asbp_teapot)))

(event Custom|Activate
  (params (Teapot :type BP%20Teapot%20Object%20Reference))
  (if (not (Variables|Default|GetActivated?))
    (Variables|Default|SetActivated? true)
    (Default|AddActivatedPoint (Variables|/Game/Blueprints/BP_Teapot.BP_Teapot_C|GetPlayerStatistics Teapot))))

(event Custom|Deactivate
  (Variables|Default|SetActivated? false))

(event EventBeginPlay)

(event Collision|EventActorBeginOverlap
  (params (OtherActor :type Actor%20Object%20Reference)))

(event EventTick
  (params (DeltaSeconds :type Float%20%28single-precision%29)))

(fn ConstructionScript
  (Components|Sphere|SetSphereRadius (Variables|Default|GetRadius) (Variables|Default|GetActivationRadius) true))