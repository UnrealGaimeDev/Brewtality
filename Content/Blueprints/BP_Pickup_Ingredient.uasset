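; Ingredient pickup that flies to the teapot player on overlap and hands over its ingredient.
; On BeginPlay, a dynamic material on the plane takes its icon from the ingredient data table.
; Pickup runs once, stopping the wiggle and driving a timeline that arcs and scales the mesh toward the player's moving position, playing slower from farther away.
; When finished, it notifies the player's controller of a dropped ingredient and destroys itself.
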(event Custom|Pickup
  (params (Player :type BP%20Teapot%20Object%20Reference))
  (if (not (Variables|Default|GetPickedUp?))
    (Variables|Default|SetPickedUp? true)
    (Audio|Components|Audio|Stop (Variables|Default|GetWiggle))
    (Variables|Default|SetPlayer Player)
    (Variables|Default|SetOriginalLocation (Transformation|GetWorldLocation (Variables|Character|GetMesh)))
    (Variables|Default|SetOriginalScale (Variables|/Script/Engine.SceneComponent|GetRelativeScale3D (Variables|Character|GetMesh)))
    (Components|Timeline|SetPlayRate (Variables|Default|GetTimeline) (Math|Float|Lerp 1.0 0.25 (Math|Float|Clamp(Float) (/ (Math|Vector|Distance(Vector) (Variables|Default|GetOriginalLocation) (Transformation|GetActorLocation (Variables|Default|GetPlayer))) 2e+03))))
    (bind (_direction _distance _zoffset _scale) (Timeline|Timeline PlayFromStart)
      (:Update
        (Transformation|SetWorldLocation (Variables|Character|GetMesh) (+ (Math|Vector|Lerp(Vector) (Transformation|GetActorLocation (Variables|Default|GetPlayer)) (Variables|Default|GetOriginalLocation) _distance) (Math|Vector|MakeVector 0.0 0.0 (Math|Float|Lerp 0.0 (Variables|Default|GetMaxZOffset) _zoffset))) false false)
        (Transformation|SetRelativeScale3D (Variables|Character|GetMesh) (* (Variables|Default|GetOriginalScale) _scale)))
      (:Finished
        (Default|OnIngredientChosen (Variables|/Game/Blueprints/BP_Teapot.BP_Teapot_C|GetControllerRef (Variables|Default|GetPlayer)) (Variables|Default|GetIngredient) true)
        (Actor|DestroyActor)))))

(event EventBeginPlay
  (bind _plane (Variables|Default|GetPlane))
  (|CallParentFunction)
  (bind _returnvalue (Rendering|Material|CreateDynamicMaterialInstance _plane 0 (Rendering|Material|GetMaterial _plane 0) "None" :!class /Script/Engine.PrimitiveComponent))
  (bind _returnvalue_2 (Utilities|GetDataTableRow "/Game/Blueprints/DataTables/DT_Ingredients.DT_Ingredients" (Variables|Default|GetIngredient))
    (:then
      (Rendering|Material|SetTextureParameterValue _returnvalue "Icon" (Utilities|Struct|BreakS_Ingredient _returnvalue_2)))))

(event Collision|EventActorBeginOverlap
  (params (OtherActor :type Actor%20Object%20Reference))
  (|CallParentFunction OtherActor) ; This node is disabled and will not be called.\nDrag off pins to build functionality.
)

(event EventTick
  (params (DeltaSeconds :type Float%20%28single-precision%29))
  (|CallParentFunction DeltaSeconds) ; This node is disabled and will not be called.\nDrag off pins to build functionality.
)

(event EventOnOverlap
  (params (Actor :type Actor%20Object%20Reference))
  (|CallParentFunction Actor)
  (bind _asbp_teapot (Utilities|Casting|CastToBP_Teapot Actor))
  (CallFunction|Pickup _asbp_teapot))

(fn ConstructionScript
  (|CallParentFunction))