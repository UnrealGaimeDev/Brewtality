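; Health pickup actor that restores a percentage of max health to a BP_Teapot that overlaps it and can regenerate health.
; Pickup fires once, then a Timeline flies the mesh and particle system to the player along an arc with a height offset, scaling them as they travel.
; Playback rate slows with distance to the player.
; When the Timeline finishes, it applies the heal from CharacterStats and destroys the actor.
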(event Custom|Pickup
  (params (Player :type BP%20Teapot%20Object%20Reference))
  (bind _particlesystem (Variables|Default|GetParticleSystem))
  (if (not (Variables|Default|GetPickedUp?))
    (Variables|Default|SetPickedUp? true)
    (Variables|Default|SetPlayer Player)
    (Variables|Default|SetOriginalLocation (Transformation|GetWorldLocation _particlesystem))
    (Variables|Default|SetOriginalScale (Variables|/Script/Engine.SceneComponent|GetRelativeScale3D _particlesystem))
    (Components|Timeline|SetPlayRate (Variables|Default|GetTimeline) (Math|Float|Lerp 1.0 0.25 (Math|Float|Clamp(Float) (/ (Math|Vector|Distance(Vector) (Variables|Default|GetOriginalLocation) (Transformation|GetActorLocation (Variables|Default|GetPlayer))) 2e+03))))
    (bind (_direction _distance _zoffset _scale) (Timeline|Timeline PlayFromStart)
      (:Update
        (Transformation|SetWorldLocation (Variables|Character|GetMesh) (+ (Math|Vector|Lerp(Vector) (Transformation|GetActorLocation (Variables|Default|GetPlayer)) (Variables|Default|GetOriginalLocation) _distance) (Math|Vector|MakeVector 0.0 0.0 (Math|Float|Lerp 0.0 (Variables|Default|GetMaxZOffset) _zoffset))) false false)
        (Transformation|SetRelativeScale3D (Variables|Character|GetMesh) (* (Variables|Default|GetOriginalScale) _scale)))
      (:Finished
        (bind _value (Default|GetMaxValue (Variables|/Game/Blueprints/BP_Teapot.BP_Teapot_C|GetCharacterStats (Variables|Default|GetPlayer)) "health"))
        (Default|RegenerateHealth (Variables|Default|GetPlayer) (* _value (/ (Math|Conversions|ToFloat(Integer) (Variables|Default|GetRegPercentage)) 1e+02)))
        (Actor|DestroyActor)))))

(event EventBeginPlay
  (|CallParentFunction) ; This node is disabled and will not be called.\nDrag off pins to build functionality.
)

(event Collision|EventActorBeginOverlap
  (params (OtherActor :type Actor%20Object%20Reference))
  (|CallParentFunction OtherActor) ; This node is disabled and will not be called.\nDrag off pins to build functionality.
)

(event EventTick
  (params (DeltaSeconds :type Float%20%28single-precision%29))
  (|CallParentFunction DeltaSeconds) ; This node is disabled and will not be called.\nDrag off pins to build functionality.
)

(event EventOnOverlap
  (params (Actor :type Actor%20Object%20Reference))
  (|CallParentFunction Actor)
  (bind _asbp_teapot (Utilities|Casting|CastToBP_Teapot Actor))
  (bind _out_ (Default|CanRegenerateHealth _asbp_teapot))
  (if _out_
    (CallFunction|Pickup _asbp_teapot)))

(fn ConstructionScript
  (|CallParentFunction))