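; BP_DotDamage is a spawned actor that applies damage over time to one afflicted actor.
; Initialize stores the damage info and starts a looping tick timer plus a duration timer, which ResetEffect restarts.
; Each tick sends an equal share of the total damage via interface message, rolling separately for critical hits.
; On expiry or an invalid target, it clears the target's DoT reference if possible and destroys itself.
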(event Custom|Initialize
  (params (Damage :type S%20Dot%20Damage%20Structure) (InflictedActor :type Actor%20Object%20Reference))
  (Variables|Default|SetDamageInfo Damage)
  (Variables|Default|SetAfflicted InflictedActor)
  (bind _returnvalue (Utilities|Time|SetTimerbyEvent (delegate Custom|EndEffect) (.Duration (Utilities|Struct|BreakS_DotDamage (Variables|Default|GetDamageInfo)))))
  (Variables|Default|SetDurationTimer _returnvalue)
  (bind _returnvalue_2 (Utilities|Time|SetTimerbyEvent (delegate Custom|OnEffectTick) (.TickInterval (Utilities|Struct|BreakS_DotDamage (Variables|Default|GetDamageInfo))) true))
  (Variables|Default|SetTickTimer _returnvalue_2))

(event Custom|EndEffect
  (bind _afflicted (Variables|Default|GetAfflicted))
  (Utilities|IsValid _afflicted
    (:Is%20Valid
      (Class|IDamageable|SetDotActor(Message) _afflicted))
    (:Is%20Not%20Valid
      _))
  (Actor|DestroyActor))

(event Custom|ResetEffect
  (Utilities|Time|ClearandInvalidateTimerbyHandle (Variables|Default|GetDurationTimer))
  (bind _returnvalue (Utilities|Time|SetTimerbyEvent (delegate Custom|EndEffect) (.Duration (Utilities|Struct|BreakS_DotDamage (Variables|Default|GetDamageInfo)))))
  (Variables|Default|SetDurationTimer _returnvalue))

(event Custom|OnEffectTick
  (bind _afflicted (Variables|Default|GetAfflicted))
  (bind _damageinfo (Variables|Default|GetDamageInfo))
  (bind (_amount _duration _tickinterval _sourcetype _sourceactor _critchance _critmultiplier) (Utilities|Struct|BreakS_DotDamage _damageinfo))
  (bind _returnvalue (/ _duration _tickinterval))
  (bind _returnvalue_2 (/ _amount _returnvalue))
  (Utilities|IsValid _afflicted
    (:Is%20Valid
      (bind _out (CallFunction|RandomBoolfromChance _critchance))
      (if _out
        (Class|IDamageable|ReceiveDamage(Message) _afflicted (Utilities|Struct|MakeS_Damage (* _returnvalue_2 _critmultiplier) _sourcetype _sourceactor 0.0 true "NewEnumerator1"))
        (else
          (Class|IDamageable|ReceiveDamage(Message) _afflicted (Utilities|Struct|MakeS_Damage _returnvalue_2 "NewEnumerator0" _sourceactor 0.0 false "NewEnumerator1")))))
    (:Is%20Not%20Valid
      (CallFunction|EndEffect))))

(fn ConstructionScript)