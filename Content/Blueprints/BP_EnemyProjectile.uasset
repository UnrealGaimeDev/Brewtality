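; Enemy projectile actor that damages the first valid target it overlaps and destroys itself on impact.
; The construction script feeds its speed into ProjectileMovement, and collision hits destroy it outright.
; Overlaps query I_Damageable before sending DamageInfo, with a HasCollided flag preventing repeat damage.
; A looping timer checks distance from the spawn origin and, beyond max range, spawns a Niagara end effect before destroying it.
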(event OnComponentHit(Collision)
  (params (HitComponent :type Primitive%20Component%20Object%20Reference) (OtherActor :type Actor%20Object%20Reference) (OtherComp :type Primitive%20Component%20Object%20Reference) (NormalImpulse :type Vector :default "0, 0, 0") (Hit :type Hit%20Result%20Structure%20%28by%20ref%29))
  (CallFunction|DestroyProjectile))

(event OnComponentBeginOverlap(Collision)
  (params (OverlappedComponent :type Primitive%20Component%20Object%20Reference) (OtherActor :type Actor%20Object%20Reference) (OtherComp :type Primitive%20Component%20Object%20Reference) (OtherBodyIndex :type Integer) (bFromSweep :type Boolean) (SweepResult :type Hit%20Result%20Structure%20%28by%20ref%29))
  (if (not (Variables|Default|GetHasCollided?))
    (if (Utilities|DoesObjectImplementInterface OtherActor "/Game/Blueprints/Interfaces/I_Damageable.I_Damageable_C")
      (bind _out_ (Class|IDamageable|CanReceiveDamage?(Message) OtherActor (Variables|Default|GetDamageInfo)))
      (if _out_
        (Variables|Default|SetHasCollided? true)
        (Utilities|Set|Add (Variables|Default|GetHitActors) OtherActor)
        (Class|IDamageable|ReceiveDamage(Message) OtherActor (Variables|Default|GetDamageInfo))
        (CallFunction|DestroyProjectile)))))

(event Custom|DestroyProjectile
  (Actor|DestroyActor))

(event EventBeginPlay
  (Variables|Default|SetOrigin (Transformation|GetActorLocation))
  (bind _returnvalue (Utilities|Time|SetTimerbyFunctionName 0 "CheckTravelDistance" 0.25 true))
  (Variables|Default|SetTravelTimer _returnvalue))

(fn ConstructionScript
  (Variables|/Script/Engine.ProjectileMovementComponent|SetInitialSpeed (Variables|Default|GetProjectileMovement) (Variables|Default|GetProjectileSpeed)))

(fn CheckTravelDistance
  (if (and (>= (Math|Vector|Distance(Vector) (Transformation|GetActorLocation) (Variables|Default|GetOrigin)) (Variables|Default|GetMaxTravelDistance)) (not (Variables|Default|GetHasCollided?)))
    (Niagara|SpawnSystematLocation "/Game/VFX/NS_ProjectileLifeEnd.NS_ProjectileLifeEnd" (Transformation|GetActorLocation) (Transformation|GetActorRotation))
    (CallFunction|DestroyProjectile)))