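; Master projectile that damages I_Damageable actors on overlap or hit, skipping those already hit, with optional ricochet and passthrough.
; Ricochets take priority, using a sphere trace to aim at the first damageable actor found, otherwise reversing direction.
; Passthrough overlaps all channels and scales down damage and knockback after each damaging hit.
; A looping timer expires it beyond max travel distance, and a timeline stretches the mesh at spawn.
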(event OnComponentHit(Collision)
  (params (HitComponent :type Primitive%20Component%20Object%20Reference) (OtherActor :type Actor%20Object%20Reference) (OtherComp :type Primitive%20Component%20Object%20Reference) (NormalImpulse :type Vector :default "0, 0, 0") (Hit :type Hit%20Result%20Structure%20%28by%20ref%29))
  (CallFunction|OnProjectileHit OtherActor true))

(event OnComponentBeginOverlap(Collision)
  (params (OverlappedComponent :type Primitive%20Component%20Object%20Reference) (OtherActor :type Actor%20Object%20Reference) (OtherComp :type Primitive%20Component%20Object%20Reference) (OtherBodyIndex :type Integer) (bFromSweep :type Boolean) (SweepResult :type Hit%20Result%20Structure%20%28by%20ref%29))
  (CallFunction|OnProjectileHit OtherActor false))

(event Custom|RicochetOff
  (params (HitActor :type Actor%20Object%20Reference))
  (bind _hitactors (Variables|Default|GetHitActors))
  (Math|Integer|DecrementInt (Variables|Default|GetRicochets)
    (:%20%20
      (Utilities|Set|Clear _hitactors)
      (Utilities|Set|Add _hitactors HitActor)
      (bind _output_get (Variables|Default|SetOrigin (Transformation|GetActorLocation)))
      (Variables|Default|SetRicochetDirection (* (Variables|/Script/Engine.MovementComponent|GetVelocity (Variables|Default|GetProjectileMovement)) -1.0))
      (bind _result (Utilities|Set|ToArray (Variables|Default|GetHitActors)))
      (bind (_outhits _returnvalue) (Collision|MultiSphereTraceByChannel _output_get _output_get (+ (Variables|Default|GetMaxTravelDistance) 1e+02) "TraceTypeQuery1" false _result "None"))
      (if _returnvalue
        (bind _array_element (Utilities|Array|ForEachLoopwithBreak _outhits :!label _label)
          (:LoopBody
            (if (Utilities|DoesObjectImplementInterface (.HitActor (Collision|BreakHitResult _array_element)) "/Game/Blueprints/Interfaces/I_Damageable.I_Damageable_C")
              (bind _out_ (Class|IDamageable|CanReceiveDamage?(Message) (.HitActor (Collision|BreakHitResult _array_element)) (Variables|Default|GetDamageInfo)))
              (if _out_
                (Variables|Default|SetRicochetDirection (Math|Vector|Normalize (- (Transformation|GetActorLocation (.HitActor (Collision|BreakHitResult _array_element))) (Variables|Default|GetOrigin))))
                (goto _label Break))))
          (:Completed
            (Variables|/Script/Engine.MovementComponent|SetVelocity (Variables|Default|GetProjectileMovement) (* (Variables|Default|GetRicochetDirection) (Variables|Default|GetProjectileSpeed)) :!label _label_2)
            (Variables|Default|SetHasCollided? false)
            (Transformation|SetActorRotation (Math|Conversions|RotationFromXVector (Variables|/Script/Engine.MovementComponent|GetVelocity (Variables|Default|GetProjectileMovement))) true)))
        (else
          (goto _label_2))))))

(event Custom|OnProjectileHit
  (params (HitActor :type Actor%20Object%20Reference) (Destroy? :type Boolean))
  (bind _damageinfo (Variables|Default|GetDamageInfo))
  (bind _passthroughdamagemult (Variables|Default|GetPassthroughDamageMult))
  (bind (_amount _knockback) (Utilities|Struct|BreakS_Damage _damageinfo))
  (if (Utilities|DoesObjectImplementInterface HitActor "/Game/Blueprints/Interfaces/I_Damageable.I_Damageable_C")
    (if (Utilities|Set|Contains (Variables|Default|GetHitActors) HitActor)
      (if Destroy? :!label _label
        (Niagara|SpawnSystematLocation "/Game/VFX/NS_ProjectileExplosion.NS_ProjectileExplosion" (Transformation|GetActorLocation) (Transformation|GetActorRotation) :!label _label_2)
        (if (> (Variables|Default|GetRicochets) 0)
          (CallFunction|RicochetOff HitActor)
          (elif (Variables|Default|GetPassthrough?)
            (Variables|Default|SetHasCollided? false)
            (Utilities|Struct|SetmembersinS_Damage _damageinfo (Math|Float|Max(Float) (* _amount _passthroughdamagemult) 1.0) (* _knockback _passthroughdamagemult))
            (else
              (CallFunction|DestroyProjectile)))))
      (else
        (bind _out_ (Class|IDamageable|CanReceiveDamage?(Message) HitActor (Variables|Default|GetDamageInfo)))
        (if _out_
          (Utilities|Set|Add (Variables|Default|GetHitActors) HitActor)
          (Variables|Default|SetHasCollided? true)
          (Class|IDamageable|ReceiveDamage(Message) HitActor (Variables|Default|GetDamageInfo))
          (goto _label_2)
          (else
            (goto _label)))))
    (else
      (goto _label))))

(event Custom|DestroyProjectile
  (Actor|DestroyActor))

(event EventBeginPlay
  (bind _mesh (Variables|Default|GetMesh))
  (bind _relativescale3d (Variables|/Script/Engine.SceneComponent|GetRelativeScale3D _mesh))
  (bind (_x _y _z) (Math|Vector|BreakVector _relativescale3d))
  (CallFunction|TryPassthroughCheck)
  (Variables|Default|SetOrigin (Transformation|GetActorLocation))
  (Utilities|Time|SetTimerbyFunctionName self "CheckTravelDistance" 0.1 true)
  (Variables|Default|SetOriginalXScale (.X (Math|Vector|BreakVector (Variables|/Script/Engine.SceneComponent|GetRelativeScale3D (Variables|Default|GetMesh)))))
  (bind _xscaleperc (Timeline|Stretch PlayFromStart)
    (:Update
      (Transformation|SetRelativeScale3D _mesh (Math|Vector|MakeVector (Math|Float|Lerp (Variables|Default|GetOriginalXScale) (Variables|Default|GetStretchXScale) _xscaleperc) _y _z)))))

(fn ConstructionScript
  (Variables|/Script/Engine.ProjectileMovementComponent|SetInitialSpeed (Variables|Default|GetProjectileMovement) (Variables|Default|GetProjectileSpeed)))

(fn CheckTravelDistance
  (if (and (>= (Math|Vector|Distance(Vector) (Transformation|GetActorLocation) (Variables|Default|GetOrigin)) (Variables|Default|GetMaxTravelDistance)) (not (Variables|Default|GetHasCollided?)))
    (Niagara|SpawnSystematLocation "/Game/VFX/NS_ProjectileLifeEnd.NS_ProjectileLifeEnd" (Transformation|GetActorLocation) (Transformation|GetActorRotation))
    (CallFunction|DestroyProjectile)))

(fn TryPassthroughCheck
  (if (Variables|Default|GetPassthrough?)
    (Collision|SetCollisionResponsetoAllChannels (Variables|Default|GetCollision) "ECR_Overlap")))