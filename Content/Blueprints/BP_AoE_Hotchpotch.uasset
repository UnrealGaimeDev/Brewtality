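; Child AoE Blueprint for an expanding shockwave that grows from the triggered radius to a final radius, then ends.
; TriggerAoE runs the parent logic, then plays the Grow timeline at a rate derived from TravelSpeed and the radius difference, so expansion speed stays consistent.
; Each timeline update calls UpdateRadius, which scales the Shockwave component to the interpolated radius and passes it to the parent.
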(event EventTriggerAoE
  (params (Damage :type S%20Damage%20Structure) (Radius :type Float%20%28single-precision%29) (CritPercentage :type Float%20%28double-precision%29) (CritMultiplier :type Float%20%28double-precision%29))
  (Variables|Default|SetOriginalRadius Radius)
  (|CallParentFunction Damage Radius CritPercentage CritMultiplier)
  (Components|Timeline|SetPlayRate (Variables|Default|GetGrow) (/ 1.0 (/ (- (Variables|Default|GetFinalRadius) (Variables|Default|GetOriginalRadius)) (Variables|Default|GetTravelSpeed))))
  (bind _perc (Timeline|Grow PlayFromStart)
    (:Update
      (CallFunction|UpdateRadius (Math|Float|Lerp (Variables|Default|GetOriginalRadius) (Variables|Default|GetFinalRadius) _perc)))
    (:Finished
      (CallFunction|EndAoE))))

(fn ConstructionScript
  (|CallParentFunction))

(fn UpdateRadius
  (params (NewRadius :type Float%20%28single-precision%29))
  (Transformation|SetRelativeScale3D (Variables|Default|GetShockwave) (Math|Conversions|ToVector(Float) (/ NewRadius 32.0)))
  (|CallParentFunction NewRadius))