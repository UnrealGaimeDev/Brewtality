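; BP_Dodge is a short-lived actor that shows an animated dodge text widget following a target actor.
; On BeginPlay it reveals its DodgeWidget component, binds to the WBP_DodgeText animation-finished event and starts the animation.
; Tick keeps it at the target's location plus an offset while the target is valid, and the actor destroys itself when the animation ends.
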(event Custom|OnWidgetAnimEnd
  (Actor|DestroyActor))

(event EventBeginPlay
  (bind _aswbp_dodge_text (Utilities|Casting|CastToWBP_DodgeText (UserInterface|GetUserWidgetObject (Variables|Default|GetDodgeWidget))))
  (Rendering|SetVisibility (Variables|Default|GetDodgeWidget) true false)
  (EventDispatchers|BindEventtoOnAnimFinished _aswbp_dodge_text (delegate Custom|OnWidgetAnimEnd))
  (Default|PlayAnim _aswbp_dodge_text))

(event EventTick
  (params (DeltaSeconds :type Float%20%28single-precision%29))
  (Utilities|IsValid (Variables|Default|GetTargetActor)
    (:Is%20Valid
      (Transformation|SetActorLocation (+ (Transformation|GetActorLocation (Variables|Default|GetTargetActor)) (Variables|Default|GetOffset)) false false))))

(fn ConstructionScript)