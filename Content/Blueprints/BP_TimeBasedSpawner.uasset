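; Enemy spawner that follows the player along the Y axis and spawns weighted-random enemy batches at random intervals.
; Settings load from a DT_EnemySpawns row, and each batch enemy gets a random reachable navmesh point within the radius, found by recursive retry.
; A separate timer tracks elapsed time and applies the row's timed modifications in key order, adjusting intervals, counts and enemy weights as play progresses.
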(event Custom|DestroySpawner
  (Actor|DestroyActor))

(event Custom|SpawnEnemy
  (params (EnemyClass :type BP%20Master%20Enemy%20Class%20Reference))
  (bind _location (CallFunction|GetSpawnPoint))
  (Game|SpawnActorfromClass EnemyClass (Math|Transform|MakeTransform _location) "AdjustIfPossibleButAlwaysSpawn" "MultiplyWithRoot" 0 0))

(event Custom|SpawnTick
  (bind _spawnsettings (Variables|Default|GetSpawnSettings))
  (bind _numberofenemies (Utilities|Struct|BreakS_DefaultSpawn _spawnsettings))
  (bind (_min _max) (Utilities|Struct|BreakS_IntRange _numberofenemies))
  (bind _output_get (Variables|Default|SetNumberToSpawn (Math|Random|RandomIntegerinRange _min _max)))
  (for _index (range 0 (- _output_get -1))
    (bind _enemy (CallFunction|GetRandomEnemy))
    (if (Utilities|IsValidClass _enemy)
      (CallFunction|SpawnEnemy _enemy)))
  (CallFunction|SetTickTimer))

(event Custom|UpdatePosition
  (bind _returnvalue (Transformation|GetActorLocation))
  (bind (_x _y _z) (Math|Vector|BreakVector _returnvalue))
  (Transformation|SetActorLocation (Math|Vector|MakeVector _x (.Y (Math|Vector|BreakVector (Transformation|GetActorLocation (Game|Player|GetPlayerPawn 0)))) _z) false false))

(event Custom|SetTickTimer
  (bind _spawnsettings (Variables|Default|GetSpawnSettings))
  (bind _spawninterval (Utilities|Struct|BreakS_DefaultSpawn _spawnsettings))
  (bind (_min _max) (Utilities|Struct|BreakS_FloatRange _spawninterval))
  (bind _output_get (Variables|Default|SetTimeUntilTick (Math|Random|RandomFloatinRange _min _max)))
  (bind _returnvalue (Utilities|Time|SetTimerbyEvent (delegate Custom|SpawnTick) _output_get))
  (Variables|Default|SetTickTimer _returnvalue))

(event Custom|TimeUpdateTick
  (Variables|Default|SetPassedTime (+ (Variables|Default|GetPassedTime) (Variables|Default|GetUpdateInterval)))
  (bind (_success_ _time _modification) (CallFunction|TryGetNextMod))
  (if _success_
    (if (>= (Variables|Default|GetPassedTime) _time)
      (CallFunction|ApplyModification _modification)
      (Utilities|Map|Remove (Variables|Default|GetRemainingModifications) _time))
    (else
      (Utilities|Time|ClearandInvalidateTimerbyHandle (Variables|Default|GetTimeUpdateTimer)))))

(event EventBeginPlay
  (Utilities|FlowControl|Sequence
    (:then_0
      (Utilities|Time|SetTimerbyEvent (delegate Custom|UpdatePosition) 0.25 true)
      (Variables|Default|SetPassedTime 0.0)
      (bind _returnvalue (Utilities|Time|SetTimerbyEvent (delegate Custom|TimeUpdateTick) (Variables|Default|GetUpdateInterval) true))
      (Variables|Default|SetTimeUpdateTimer _returnvalue))
    (:then_1
      (bind _returnvalue_2 (Utilities|GetDataTableRow "/Game/Blueprints/DataTables/DT_EnemySpawns.DT_EnemySpawns" (Variables|Default|GetDatatableRow))
        (:then
          (Variables|Default|SetSpawnSettings (.DefaultSettings (Utilities|Struct|BreakS_EnemySpawn _returnvalue_2)))
          (Variables|Default|SetRemainingModifications (.TimeModifications (Utilities|Struct|BreakS_EnemySpawn _returnvalue_2)))
          (CallFunction|CalculateTotalWeights)
          (CallFunction|SetTickTimer))))))

(fn ConstructionScript
  (Components|Sphere|SetSphereRadius (Variables|Default|GetSpawnRadius) (Variables|SpawnBehaviour|GetRadius) true))

(fn GetSpawnPoint
  (params (CallNumber :type Integer))
  (bind _radius (Variables|SpawnBehaviour|GetRadius))
  (bind _spawnradius (Variables|Default|GetSpawnRadius))
  (bind _returnvalue (Transformation|GetWorldLocation _spawnradius))
  (bind (_randomlocation _returnvalue_2) (AI|Navigation|GetRandomReachablePointinRadius _returnvalue _radius 0 0))
  (if _returnvalue_2
    (return _randomlocation)
    (elif (> CallNumber 5)
      (return "0, 0, 0")
      (else
        (bind _location (CallFunction|GetSpawnPoint (+ CallNumber 1)))
        (return _location)))))

(fn GetRandomEnemy
  (LocalVariables|SetlocalRandomNumber (Math|Random|RandomFloatinRange 0.0 (Variables|Default|GetWeightsTotal)))
  (bind (_keypin _valuepin) (Utilities|Map|ForEachLoop(Map) (Utilities|Struct|BreakS_DefaultSpawn (Variables|Default|GetSpawnSettings)) :!label _label)
    (:then
      (if (<= (LocalVariables|GetlocalRandomNumber) (+ _valuepin (LocalVariables|GetlocalAdd)))
        (LocalVariables|SetlocalEnemy _keypin)
        (goto _label BreakPin)
        (else
          (LocalVariables|SetlocalAdd (+ (LocalVariables|GetlocalAdd) _valuepin)))))
    (:CompletedPin
      (return (LocalVariables|GetlocalEnemy)))))

(fn CalculateTotalWeights
  (LocalVariables|SetlocalAmount 0.0)
  (bind _valuepin (Utilities|Map|ForEachLoop(Map) (Utilities|Struct|BreakS_DefaultSpawn (Variables|Default|GetSpawnSettings)))
    (:then
      (LocalVariables|SetlocalAmount (+ _valuepin (LocalVariables|GetlocalAmount))))
    (:CompletedPin
      (Variables|Default|SetWeightsTotal (LocalVariables|GetlocalAmount)))))

(fn TryGetNextMod
  (bind _remainingmodifications (Variables|Default|GetRemainingModifications))
  (bind _keys (Utilities|Map|Keys _remainingmodifications))
  (if (Utilities|Array|IsEmpty _keys)
    (return false 0.0 "")
    (else
      (return true (Utilities|Array|Get(acopy) _keys) (.Value (Utilities|Map|Find _remainingmodifications (Utilities|Array|Get(acopy) _keys)))))))

(fn ApplyModification
  (params (Modification :type S%20Spawn%20Modifier%20Structure))
  (bind (_mininterval _maxinterval _numberofenemies _enemyweights) (Utilities|Struct|BreakS_SpawnModifier Modification))
  (bind (_flatmodifier _percentagemodifier) (Utilities|Struct|BreakS_StatModifier _mininterval))
  (bind (_flatmodifier_2 _percentagemodifier_2) (Utilities|Struct|BreakS_StatModifier _maxinterval))
  (bind (_min _max) (Utilities|Struct|BreakS_IntRange _numberofenemies))
  (bind _structout (Utilities|Struct|SetmembersinS_DefaultSpawn (Variables|Default|GetSpawnSettings) (Utilities|Struct|MakeS_FloatRange (+ (* (.Min (Utilities|Struct|BreakS_FloatRange (.SpawnInterval (Utilities|Struct|BreakS_DefaultSpawn (Variables|Default|GetSpawnSettings))))) _percentagemodifier) _flatmodifier) (+ (* (.Max (Utilities|Struct|BreakS_FloatRange (.SpawnInterval (Utilities|Struct|BreakS_DefaultSpawn (Variables|Default|GetSpawnSettings))))) _percentagemodifier_2) _flatmodifier_2)) (Utilities|Struct|MakeS_IntRange (+ (.Min (Utilities|Struct|BreakS_IntRange (.NumberOfEnemies (Utilities|Struct|BreakS_DefaultSpawn (Variables|Default|GetSpawnSettings))))) _min) (+ (.Max (Utilities|Struct|BreakS_IntRange (.NumberOfEnemies (Utilities|Struct|BreakS_DefaultSpawn (Variables|Default|GetSpawnSettings))))) _max))))
  (Variables|Default|SetSpawnSettings _structout)
  (bind _output_get (LocalVariables|SetlocalWeightsMod _enemyweights))
  (LocalVariables|SetlocalCurrentWeights (Utilities|Struct|BreakS_DefaultSpawn (Variables|Default|GetSpawnSettings)))
  (bind (_keypin _valuepin) (Utilities|Map|ForEachLoop(Map) _output_get)
    (:then
      (if (.ReturnValue (Utilities|Map|Find (LocalVariables|GetlocalCurrentWeights) _keypin))
        (bind _output_get_2 (LocalVariables|SetlocalPrevious (.Value (Utilities|Map|Find (LocalVariables|GetlocalCurrentWeights) _keypin))))
        (bind _output_get_3 (LocalVariables|SetlocalNew (+ _output_get_2 _valuepin)))
        (if (<= _output_get_3 0.0)
          (Utilities|Array|Add (LocalVariables|GetlocalClassesToRemove) _keypin)
          (else
            (Utilities|Map|Add (LocalVariables|GetlocalCurrentWeights) _keypin (LocalVariables|GetlocalNew))))
        (elif (> _valuepin 0.0)
          (Utilities|Map|Add (LocalVariables|GetlocalCurrentWeights) _keypin _valuepin))))
    (:CompletedPin
      (for _array_element (LocalVariables|GetlocalClassesToRemove)
        (Utilities|Map|Remove (LocalVariables|GetlocalCurrentWeights) _array_element))
      (bind _structout_2 (Utilities|Struct|SetmembersinS_DefaultSpawn (Variables|Default|GetSpawnSettings) (LocalVariables|GetlocalCurrentWeights)))
      (Variables|Default|SetSpawnSettings _structout_2)
      (CallFunction|CalculateTotalWeights)
      (return))))