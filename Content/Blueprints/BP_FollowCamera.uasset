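; BP_FollowCamera is a camera actor that becomes player 0's view target on BeginPlay and follows that player's pawn in the XY plane.
; Each Tick it moves to the pawn's X and Y while keeping the Z height recorded at BeginPlay.
; With UseBounds enabled, X is clamped to the XBounds range and Y is only limited from below by YLimit.
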(event EventBeginPlay
  (Game|Player|SetViewTargetwithBlend (Game|GetPlayerController 0) self 0.0 "VTBlend_Linear" 0.0 false)
  (Variables|Default|SetOriginalLocation (Transformation|GetActorLocation)))

(event EventTick
  (params (DeltaSeconds :type Float%20%28single-precision%29))
  (bind _returnvalue (Game|Player|GetPlayerPawn 0))
  (bind _returnvalue_2 (Game|Player|GetPlayerPawn 0))
  (bind _xbounds (Variables|Default|GetXBounds))
  (bind (_min _max) (Utilities|Struct|BreakS_Bounds _xbounds))
  (bind _returnvalue_3 (Transformation|GetActorLocation _returnvalue_2))
  (bind _returnvalue_4 (Transformation|GetActorLocation _returnvalue))
  (bind (_x _y) (Math|Vector|BreakVector _returnvalue_3))
  (bind (_x_2 _y_2) (Math|Vector|BreakVector _returnvalue_4))
  (if (Variables|Default|GetUseBounds?)
    (Transformation|SetActorLocation (Math|Vector|MakeVector (Math|Float|Clamp(Float) _x _min _max) (Math|Float|Max(Float) _y (Variables|Default|GetYLimit)) (.Z (Math|Vector|BreakVector (Variables|Default|GetOriginalLocation)))) false false)
    (else
      (Transformation|SetActorLocation (Math|Vector|MakeVector _x_2 _y_2 (.Z (Math|Vector|BreakVector (Variables|Default|GetOriginalLocation)))) false false))))

(fn ConstructionScript)