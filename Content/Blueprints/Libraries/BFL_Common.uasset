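; Blueprint function library of small shared helpers for vector math, chance rolls, ground detection and sound.
; It flattens a vector's Z, rolls a percent chance, and finds ground under an actor with a downward WorldStatic line trace from above it, returning zero on a miss.
; Sound helpers validate the asset, then either play it or spawn an audio component, as 2D or at a location.
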(fn RemoveZ
  (params (In :type Vector))
  (return (Math|Vector|MakeVector (.x In) (.y In) 0.0)))

(fn RandomBoolfromChance
  (params (TrueChance :type Float%20%28double-precision%29))
  (if (< (Math|Random|RandomFloatinRange 0.0 1e+02) TrueChance)
    (return true)
    (else
      (return false))))

(fn FindGroundLocation
  (params (Actor :type Actor%20Object%20Reference))
  (bind _returnvalue (Transformation|GetActorLocation Actor))
  (bind (_outhit _returnvalue_2) (Collision|LineTraceForObjects Actor (+ _returnvalue "0.000000,0.000000,1000.000000") (+ _returnvalue (* (Math|Vector|VectorDown) 1e+04)) (Utilities|Array|MakeArray "ObjectTypeQuery1") false (Utilities|Array|MakeArray Actor) "None"))
  (if _returnvalue_2
    (return (.Location (Collision|BreakHitResult _outhit)))
    (else
      (return "0, 0, 0"))))

(fn PlaySound
  (params (Sound :type Sound%20Base%20Object%20Reference) (AtLocation? :type Boolean) (Location :type Vector))
  (Utilities|IsValid Sound
    (:Is%20Valid
      (if AtLocation?
        (Audio|PlaySoundatLocation 0 Sound Location "0, 0, 0" 1.0 1.0 0.0 0 0 0 0)
        (return)
        (else
          (Audio|PlaySound2D 0 Sound 1.0 1.0 0.0 0 0)
          (return))))
    (:Is%20Not%20Valid
      (return))))

(fn CreateSound
  (params (Sound :type Sound%20Base%20Object%20Reference) (AtLocation? :type Boolean) (Location :type Vector))
  (Utilities|IsValid Sound
    (:Is%20Valid
      (if AtLocation?
        (bind _returnvalue (Audio|SpawnSoundatLocation 0 Sound Location "0, 0, 0" 1.0 1.0 0.0 0 0))
        (return _returnvalue)
        (else
          (bind _returnvalue_2 (Audio|SpawnSound2D 0 Sound 1.0 1.0 0.0 0))
          (return _returnvalue_2))))
    (:Is%20Not%20Valid
      (return 0))))