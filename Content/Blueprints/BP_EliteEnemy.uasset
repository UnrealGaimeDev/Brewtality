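; BP_EliteEnemy is an enemy variant that adds camera feedback when it dies.
; On death it casts the first player controller to BP_TeapotController and plays the boss-kill camera shake at the mesh location, attenuated by distance.
; The parent death logic then runs through a sequence, so it still executes if the cast fails.
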(event EventBeginPlay
  (|CallParentFunction) ; This node is disabled and will not be called.\nDrag off pins to build functionality.
)

(event Collision|EventActorBeginOverlap
  (params (OtherActor :type Actor%20Object%20Reference)))

(event EventTick
  (params (DeltaSeconds :type Float%20%28single-precision%29)))

(event EventOnDeath
  (params (ByKill? :type Boolean))
  (Utilities|FlowControl|Sequence
    (:then_0
      (bind _asbp_teapot_controller (Utilities|Casting|CastToBP_TeapotController (Game|GetPlayerController 0)))
      (Default|PlayerCameraShakeatLocation _asbp_teapot_controller "/Game/Feedback/CS_BossKill.CS_BossKill_C" (Transformation|GetWorldLocation (Variables|Character|GetMesh)) 5e+02 1.5e+03 1.0))
    (:then_1
      (|CallParentFunction ByKill?))))

(fn ConstructionScript
  (|CallParentFunction))