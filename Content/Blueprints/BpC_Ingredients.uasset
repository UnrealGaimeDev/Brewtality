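; Ingredient component for the Teapot that tracks collected ingredients, updates the main widget and applies their DT_Ingredients stat and base/max modifiers.
; Builds a weighted pool by repeating each available ingredient by rarity, plus luck-scaled copies for owned ingredients unless exempt.
; Selections shuffle a pool copy minus exclusions and remove each pick to avoid repeats.
; Adding, unlocking or removing ingredients from availability rebuilds the pool.
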(event Custom|Initialize
  (params (Teapot :type BP%20Teapot%20Object%20Reference))
  (Variables|Default|SetTeapot Teapot)
  (CallFunction|GenerateTotalPool))

(event Custom|OnIngredientChosen
  (params (Ingredient :type Name))
  (CallFunction|AddIngredient Ingredient)
  (CallFunction|ApplyIngredient Ingredient))

(fn GetIngredientInfo
  (params (Ingredient :type Name))
  (bind _returnvalue (Utilities|GetDataTableRow "/Game/Blueprints/DataTables/DT_Ingredients.DT_Ingredients" Ingredient)
    (:then
      (return true _returnvalue))
    (:RowNotFound
      (return false ""))))

(fn GenerateTotalPool
  (bind _teapot (Variables|Default|GetTeapot))
  (Utilities|IsValid _teapot
    (:Is%20Valid
      (bind _value (Default|GetFinalValue (Variables|/Game/Blueprints/BP_Teapot.BP_Teapot_C|GetCharacterStats _teapot) "luck"))
      (LocalVariables|SetlocalLuck _value))
    (:Is%20Not%20Valid
      _))
  (Utilities|Array|Clear (Variables|Pool|GetTotalPool))
  (for _array_element (Variables|Progression|GetAvailableIngredients)
    (LocalVariables|SetlocalIngredient _array_element)
    (bind (_found_ _info) (CallFunction|GetIngredientInfo (LocalVariables|GetlocalIngredient)))
    (if _found_
      (if (.ReturnValue (Utilities|Map|Find (Variables|Finetuning|GetRarityWeights) (.Rarity (Utilities|Struct|BreakS_Ingredient _info))))
        (LocalVariables|SetlocalAmount (.Value (Utilities|Map|Find (Variables|Finetuning|GetRarityWeights) (.Rarity (Utilities|Struct|BreakS_Ingredient _info)))))
        (if (Utilities|Set|Contains (Variables|Luck|GetLuckUnaffectedIngredients) (LocalVariables|GetlocalIngredient))
          _
          (else
            (LocalVariables|SetlocalAmount (+ (LocalVariables|GetlocalAmount) (Math|Float|Round (* (.Value (Utilities|Map|Find (Variables|Default|GetIngredients) (LocalVariables|GetlocalIngredient))) (* (/ (LocalVariables|GetlocalLuck) 1e+02) (Variables|Luck|GetMaxLuckAddsPerIngredient))))))))
        (for _index (range 1 (LocalVariables|GetlocalAmount))
          (Utilities|Array|Add (Variables|Pool|GetTotalPool) (LocalVariables|GetlocalIngredient)))))))

(fn PrintTotalPool
  (for _array_element (Variables|Pool|GetTotalPool)
    (Development|PrintString (Utilities|String|ToString(Name) _array_element) true true "(R=0.000000,G=0.660000,B=1.000000,A=1.000000)" 5.0)))

(fn GenerateSelection
  (params (Number :type Integer) (Exclude :type Array%20of%20Names))
  (LocalVariables|SetlocalPool (Variables|Pool|GetTotalPool))
  (for _array_element Exclude
    (Utilities|Array|RemoveItem (LocalVariables|GetlocalPool) _array_element))
  (Utilities|Array|Shuffle (LocalVariables|GetlocalPool))
  (for _index (range 0 (- Number 1))
    (Utilities|Array|Add (LocalVariables|GetlocalSelection) (Utilities|Array|Get(acopy) (LocalVariables|GetlocalPool)))
    (Utilities|Array|RemoveItem (LocalVariables|GetlocalPool) (Utilities|Array|Get(acopy) (LocalVariables|GetlocalPool))))
  (return (LocalVariables|GetlocalSelection)))

(fn ApplyIngredient
  (params (Name :type Name))
  (bind _teapot (Variables|Default|GetTeapot))
  (bind _characterstats (Variables|/Game/Blueprints/BP_Teapot.BP_Teapot_C|GetCharacterStats _teapot))
  (bind (_found_ _info) (CallFunction|GetIngredientInfo Name))
  (if _found_
    (bind _keys (Utilities|Map|Keys (.StatModifiers (Utilities|Struct|BreakS_Ingredient _info))))
    (for _array_element _keys
      (Default|AddStatModifier (Variables|/Game/Blueprints/BP_Teapot.BP_Teapot_C|GetCharacterStats (Variables|Default|GetTeapot)) _array_element (.Value (Utilities|Map|Find (.StatModifiers (Utilities|Struct|BreakS_Ingredient _info)) _array_element))))
    (bind _keys_2 (Utilities|Map|Keys (.BaseModifiers (Utilities|Struct|BreakS_Ingredient _info))))
    (for _array_element_2 _keys_2
      (Default|ModifyMaxValue _characterstats _array_element_2 (.MaxModifier (Utilities|Struct|BreakS_BaseModifier (.Value (Utilities|Map|Find (.BaseModifiers (Utilities|Struct|BreakS_Ingredient _info)) _array_element_2)))))
      (Default|ModifyBaseValue _characterstats _array_element_2 (.BaseModifier (Utilities|Struct|BreakS_BaseModifier (.Value (Utilities|Map|Find (.BaseModifiers (Utilities|Struct|BreakS_Ingredient _info)) _array_element_2))))))
    (return true)
    (else
      (return false))))

(fn AddIngredient
  (params (Ingredient :type Name))
  (bind _ingredients (Variables|Default|GetIngredients))
  (bind (_value _returnvalue) (Utilities|Map|Find _ingredients Ingredient))
  (if _returnvalue
    (LocalVariables|SetlocalPreviousAmount _value)
    (Utilities|Map|Add (Variables|Default|GetIngredients) Ingredient (+ (LocalVariables|GetlocalPreviousAmount) 1))
    (Default|AddIngredientDisplay (Variables|/Game/Blueprints/BP_TeapotController.BP_TeapotController_C|GetMainWidgetRef (Variables|/Game/Blueprints/BP_Teapot.BP_Teapot_C|GetControllerRef (Variables|Default|GetTeapot))) Ingredient (+ (LocalVariables|GetlocalPreviousAmount) 1))
    (else
      (Utilities|Map|Add (Variables|Default|GetIngredients) Ingredient 1)
      (Default|AddIngredientDisplay (Variables|/Game/Blueprints/BP_TeapotController.BP_TeapotController_C|GetMainWidgetRef (Variables|/Game/Blueprints/BP_Teapot.BP_Teapot_C|GetControllerRef (Variables|Default|GetTeapot))) Ingredient 1)))
  (CallFunction|GenerateTotalPool))

(fn GetIngredient
  (params (Ingredient :type Name))
  (bind _ingredients (Variables|Default|GetIngredients))
  (bind (_value _returnvalue) (Utilities|Map|Find _ingredients Ingredient))
  (if _returnvalue
    (return true _value)
    (else
      (return false 0))))

(fn UnlockIngredient
  (params (Ingredient :type Name))
  (Utilities|Array|AddUnique (Variables|Progression|GetAvailableIngredients) Ingredient)
  (CallFunction|GenerateTotalPool))

(fn RemoveIngredientfromPool
  (params (Ingredient :type Name%20%28by%20ref%29))
  (Utilities|Array|RemoveItem (Variables|Progression|GetAvailableIngredients) Ingredient)
  (CallFunction|GenerateTotalPool))