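; Player component that records per-run statistics such as damage, kills, pickups, ingredients and streaks.
; Gameplay calls simple add or set-if-higher functions, while looping one-second timers measure run time and longest stretches without moving, without dashing or at max health.
; On run end it feeds totals into card progress and maxed stats on GI_Brewtality, then saves.
; GenerateDisplay passes headline statistics to the game over screen.
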(event Custom|OnRunStarted
  (Variables|Default|SetRunStartTime (Math|DateTime|Now))
  (CallFunction|StartNoMoveTimer)
  (CallFunction|StartNoDashTimer)
  (Variables|Default|SetRunTime 0.0)
  (bind _returnvalue (Utilities|Time|SetTimerbyFunctionName 0 "RunTick" 1.0 true))
  (Variables|Default|SetRunTimer _returnvalue))

(event Custom|OnRunEnded
  (CallFunction|StopNoDashTimer)
  (CallFunction|StopNoMoveTimer)
  (Utilities|Time|ClearandInvalidateTimerbyHandle (Variables|Default|GetRunTimer))
  (Variables|Default|SetRunEndTime (Math|DateTime|Now))
  (Variables|Default|SetRunDuration (- (Variables|Default|GetRunEndTime) (Variables|Default|GetRunStartTime)))
  (bind _asgi_brewtality (Utilities|Casting|CastToGI_Brewtality (Game|GetGameInstance)))
  (Default|AddCardProgress _asgi_brewtality "damage_threshold" (Variables|Default|GetDamageDealt) "NewEnumerator0")
  (Default|AddCardProgress _asgi_brewtality "vacuum" (Math|Conversions|ToFloat(Integer) (Variables|Default|GetSugarCollected)) "NewEnumerator0")
  (Default|AddCardProgress _asgi_brewtality "shield" (Variables|Default|GetDamageTaken) "NewEnumerator1")
  (Default|AddCardProgress _asgi_brewtality "dash" (Variables|Default|GetRunTime) "NewEnumerator1")
  (Default|AddCardProgress _asgi_brewtality "magnet" (Math|Conversions|ToFloat(Integer) (Utilities|Set|Length (Variables|Default|GetChosenIngredients))) "NewEnumerator1")
  (Default|AddCardProgress _asgi_brewtality "reroll" (Math|Conversions|ToFloat(Integer) (Utilities|Set|Length (Variables|Default|GetBrewnBlends))) "NewEnumerator1")
  (Default|AddCardProgress _asgi_brewtality "split" (Math|Conversions|ToFloat(Integer) (Utilities|Set|Length (Variables|Default|GetDefeatedEnemies))) "NewEnumerator1")
  (bind _number (CallFunction|CountLegendaryIngredients))
  (Default|AddCardProgress _asgi_brewtality "infinite_slow" (Math|Conversions|ToFloat(Integer) _number) "NewEnumerator1")
  (Default|AddCardProgress _asgi_brewtality "proximity_damage" (Math|Conversions|ToFloat(Integer) (Variables|Default|GetNearbyEnemiesSlain)) "NewEnumerator0")
  (Default|AddCardProgress _asgi_brewtality "reflection" (Variables|Default|GetDodgedDamage) "NewEnumerator0")
  (Default|AddCardProgress _asgi_brewtality "knockback_damage" (Math|Conversions|ToFloat(Integer) (Variables|Default|GetLegendaryRerolls)) "NewEnumerator0")
  (Default|AddCardProgress _asgi_brewtality "shockwave" (Math|Conversions|ToFloat(Integer) (Variables|Default|GetKnockbackKills)) "NewEnumerator0")
  (Default|AddCardProgress _asgi_brewtality "thornmail" (Math|Conversions|ToFloat(Integer) (Variables|Default|GetHostileCollisions)) "NewEnumerator0")
  (Default|AddCardProgress _asgi_brewtality "seeking_projectiles" (Math|Conversions|ToFloat(Integer) (Variables|Default|GetBoilProjectiles)) "NewEnumerator1")
  (Default|AddCardProgress _asgi_brewtality "dot_spread" (Math|Conversions|ToFloat(Integer) (Variables|Default|GetSuccessiveCrits)) "NewEnumerator1")
  (Default|TryAddMaxedStats _asgi_brewtality (Variables|Default|GetMaxedStats))
  (Default|AddCardProgress _asgi_brewtality "regeneration" (Variables|Default|GetNoMoveHighest) "NewEnumerator1")
  (Default|AddCardProgress _asgi_brewtality "dash_shockwave" (Variables|Default|GetNoDashHighest) "NewEnumerator1")
  (Default|AddCardProgress _asgi_brewtality "health_drop" (Variables|Default|GetMaxHealthHighest) "NewEnumerator1")
  (Default|SaveGame _asgi_brewtality))

(event Custom|StartNoMoveTimer
  (if (not (Utilities|Time|IsValidTimerHandle (Variables|Default|GetNoMoveTimerHandle)))
    (Variables|Default|SetNoMoveCurrent 0.0)
    (bind _returnvalue (Utilities|Time|SetTimerbyFunctionName 0 "NoMoveTick" 1.0 true))
    (Variables|Default|SetNoMoveTimerHandle _returnvalue)))

(event Custom|StopNoMoveTimer
  (if (Utilities|Time|IsValidTimerHandle (Variables|Default|GetNoMoveTimerHandle))
    (Variables|Default|SetNoMoveHighest (Math|Float|Max(Float) (Variables|Default|GetNoMoveCurrent) (Variables|Default|GetNoMoveHighest)))
    (Variables|Default|SetNoMoveCurrent 0.0)
    (Utilities|Time|ClearandInvalidateTimerbyHandle (Variables|Default|GetNoMoveTimerHandle))))

(event Custom|StartNoDashTimer
  (if (not (Utilities|Time|IsValidTimerHandle (Variables|Default|GetNoDashTimerHandle)))
    (Variables|Default|SetNoDashCurrent 0.0)
    (bind _returnvalue (Utilities|Time|SetTimerbyFunctionName 0 "NoDashTick" 1.0 true))
    (Variables|Default|SetNoDashTimerHandle _returnvalue)))

(event Custom|StopNoDashTimer
  (if (Utilities|Time|IsValidTimerHandle (Variables|Default|GetNoDashTimerHandle))
    (Variables|Default|SetNoDashHighest (Math|Float|Max(Float) (Variables|Default|GetNoDashHighest) (Variables|Default|GetNoDashCurrent)))
    (Variables|Default|SetNoDashCurrent 0.0)
    (Utilities|Time|ClearandInvalidateTimerbyHandle (Variables|Default|GetNoDashTimerHandle))))

(event Custom|StartMaxHealthTimer
  (if (not (Utilities|Time|IsValidTimerHandle (Variables|Default|GetMaxHealthTimerHandle)))
    (Variables|Default|SetMaxHealthCurrent 0.0)
    (bind _returnvalue (Utilities|Time|SetTimerbyFunctionName 0 "MaxHealthTick" 1.0 true))
    (Variables|Default|SetMaxHealthTimerHandle _returnvalue)))

(event Custom|StopMaxHealthTimer
  (if (Utilities|Time|IsValidTimerHandle (Variables|Default|GetMaxHealthTimerHandle))
    (Variables|Default|SetMaxHealthHighest (Math|Float|Max(Float) (Variables|Default|GetMaxHealthCurrent) (Variables|Default|GetMaxHealthHighest)))
    (Variables|Default|SetMaxHealthCurrent 0.0)
    (Utilities|Time|ClearandInvalidateTimerbyHandle (Variables|Default|GetMaxHealthTimerHandle))))

(fn AddDamageDealt
  (params (Modifier :type Float%20%28double-precision%29))
  (Variables|Default|SetDamageDealt (+ Modifier (Variables|Default|GetDamageDealt))))

(fn AddLevelReached
  (params (Modifier :type Integer))
  (Variables|Default|SetLevelReached (+ Modifier (Variables|Default|GetLevelReached))))

(fn AddEnemiesKilled
  (params (Modifier :type Integer) (Nearby? :type Boolean))
  (Variables|Default|SetEnemiesKilled (+ Modifier (Variables|Default|GetEnemiesKilled)))
  (if Nearby?
    (Variables|Default|SetNearbyEnemiesSlain (+ (Variables|Default|GetNearbyEnemiesSlain) 1))))

(fn GenerateDisplay
  (params (GameOverScreen :type WBP%20Gameover%20Object%20Reference))
  (for (_array_element _array_index) (Variables|Default|GetStatistics)
    (Default|AddStatistic GameOverScreen (Utilities|Struct|MakeS_StatisticDisplay (Utilities|Struct|BreakS_StatisticDisplay _array_element) (Utilities|Select :Index _array_index :Option%200 (Class|KismetTextLibrary|AsTimespanTimespan (Variables|Default|GetRunDuration)) :Option%201 (Utilities|Text|ToText(Integer) (Variables|Default|GetLevelReached)) :Option%202 (Utilities|Text|ToText(Integer) (Variables|Default|GetEnemiesKilled)) :Option%203 (Utilities|Text|ToText(Float) (Variables|Default|GetDamageDealt) "HalfToEven" false true 1 324 0 2)))))
  (return))

(fn AddSugarCollected
  (Variables|Default|SetSugarCollected (+ (Variables|Default|GetSugarCollected) 1)))

(fn AddDamageTaken
  (params (Amount :type Float%20%28double-precision%29))
  (Variables|Default|SetDamageTaken (+ (Variables|Default|GetDamageTaken) Amount)))

(fn AddChosenIngredient
  (params (Ingredient :type Name%20%28by%20ref%29))
  (Utilities|Set|Add (Variables|Default|GetChosenIngredients) Ingredient))

(fn AddBrewnBlend
  (params (Blend :type Name%20%28by%20ref%29))
  (Utilities|Set|Add (Variables|Default|GetBrewnBlends) Blend))

(fn AddDefeatedEnemy
  (params (EnemyClass :type BP%20Master%20Enemy%20Class%20Reference%20%28by%20ref%29))
  (Utilities|Set|Add (Variables|Default|GetDefeatedEnemies) EnemyClass))

(fn CountLegendaryIngredients
  (bind _result (Utilities|Set|ToArray (Variables|Default|GetChosenIngredients)))
  (for _array_element _result
    (bind _returnvalue (Utilities|GetDataTableRow "/Game/Blueprints/DataTables/DT_Ingredients.DT_Ingredients" _array_element)
      (:then
        (switch Utilities|FlowControl|Switch|SwitchonE_Rarities (Utilities|Struct|BreakS_Ingredient _returnvalue)
          (:NewEnumerator2
            (LocalVariables|SetlocalNumber (+ (LocalVariables|GetlocalNumber) 1)))))))
  (return (LocalVariables|GetlocalNumber)))

(fn AddDodgedDamage
  (params (Amount :type Float%20%28double-precision%29))
  (Variables|Default|SetDodgedDamage (+ (Variables|Default|GetDodgedDamage) Amount)))

(fn AddLegendaryReroll
  (Variables|Default|SetLegendaryRerolls (+ (Variables|Default|GetLegendaryRerolls) 1)))

(fn AddKnockbackKill
  (Variables|Default|SetKnockbackKills (+ (Variables|Default|GetKnockbackKills) 1)))

(fn AddEnemyCollision
  (Variables|Default|SetHostileCollisions (+ (Variables|Default|GetHostileCollisions) 1)))

(fn TrySetBoilProjectiles
  (params (Amount :type Integer))
  (if (> Amount (Variables|Default|GetBoilProjectiles))
    (Variables|Default|SetBoilProjectiles Amount)))

(fn TrySetSuccessiveCrits
  (params (Amount :type Integer))
  (if (> Amount (Variables|Default|GetSuccessiveCrits))
    (Variables|Default|SetSuccessiveCrits Amount)))

(fn AddMaxedStat
  (params (Stat :type String%20%28by%20ref%29))
  (Utilities|Array|Add (Variables|Default|GetMaxedStats) Stat))

(fn NoMoveTick
  (Variables|Default|SetNoMoveCurrent (+ (Variables|Default|GetNoMoveCurrent) 1.0)))

(fn RunTick
  (Variables|Default|SetRunTime (+ (Variables|Default|GetRunTime) 1.0)))

(fn NoDashTick
  (Variables|Default|SetNoDashCurrent (+ (Variables|Default|GetNoDashCurrent) 1.0)))

(fn MaxHealthTick
  (Variables|Default|SetMaxHealthCurrent (+ (Variables|Default|GetMaxHealthCurrent) 1.0)))