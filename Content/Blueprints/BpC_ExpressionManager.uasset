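; Expression manager component that switches a mesh's displayed expression through a dynamic material instance created on a given slot.
; Expressions are added to or removed from a duplicate-free queue kept sorted by a priority map.
; The last, highest-priority entry is shown, with the default expression restored when the queue empties.
; Each expression maps to X/Y coordinates written to the ExpressionX and ExpressionY material parameters.
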(event Custom|Initialize
  (params (Mesh :type Skeletal%20Mesh%20Component%20Object%20Reference) (MaterialSlot :type Integer))
  (Utilities|IsValid Mesh
    (:Is%20Valid
      (bind _returnvalue (Rendering|Material|CreateDynamicMaterialInstance Mesh MaterialSlot (Rendering|Material|GetMaterial Mesh MaterialSlot) "None" :!class /Script/Engine.PrimitiveComponent))
      (Variables|Default|SetDynamicMaterial _returnvalue)
      (CallFunction|ResetExpression))))

(fn GetExpressionCoordinates
  (params (Expression :type E_Expressions%20Enum%20%28by%20ref%29 :default "NewEnumerator4"))
  (bind _expressioncoordinates (Variables|Default|GetExpressionCoordinates))
  (bind (_value _returnvalue) (Utilities|Map|Find _expressioncoordinates Expression))
  (if _returnvalue
    (return _value)
    (else
      (return (Utilities|Struct|MakeS_Coordinates -1 -1)))))

(fn UpdateExpressionDisplay
  (bind _dynamicmaterial (Variables|Default|GetDynamicMaterial))
  (bind _coordinates (CallFunction|GetExpressionCoordinates (Variables|Default|GetCurrentExpression)))
  (Rendering|Material|SetScalarParameterValue _dynamicmaterial "ExpressionX" (Math|Conversions|ToFloat(Integer) (.X (Utilities|Struct|BreakS_Coordinates _coordinates))) :!class /Script/Engine.MaterialInstanceDynamic)
  (Rendering|Material|SetScalarParameterValue _dynamicmaterial "ExpressionY" (Math|Conversions|ToFloat(Integer) (.Y (Utilities|Struct|BreakS_Coordinates _coordinates))) :!class /Script/Engine.MaterialInstanceDynamic))

(fn ResetExpression
  (CallFunction|SetExpression (Variables|Default|GetDefaultExpression)))

(fn SetExpression
  (params (NewExpression :type E_Expressions%20Enum :default "NewEnumerator4"))
  (if (Utilities|Enum|NotEqual(Enum) NewExpression (Variables|Default|GetCurrentExpression))
    (Variables|Default|SetCurrentExpression NewExpression)
    (CallFunction|UpdateExpressionDisplay)))

(fn AddExpression
  (params (Expression :type E_Expressions%20Enum :default "NewEnumerator4"))
  (if (Utilities|Array|IsEmpty (Variables|Default|GetExpressionQueue))
    (Utilities|Array|Add (Variables|Default|GetExpressionQueue) Expression)
    (CallFunction|OnQueueUpdated)
    (elif (Utilities|Array|ContainsItem (Variables|Default|GetExpressionQueue) Expression)
      _
      (else
        (LocalVariables|SetlocalExpression Expression)
        (LocalVariables|SetlocalIndex (Utilities|Array|Length (Variables|Default|GetExpressionQueue)))
        (bind (_array_element _array_index) (Utilities|Array|ForEachLoopwithBreak (Variables|Default|GetExpressionQueue) :!label _label)
          (:LoopBody
            (Utilities|CompareExpressions (LocalVariables|GetlocalExpression) _array_element
              (:<
                (LocalVariables|SetlocalIndex _array_index)
                (goto _label Break))))
          (:Completed
            (Utilities|Array|Insert (Variables|Default|GetExpressionQueue) (LocalVariables|GetlocalExpression) (LocalVariables|GetlocalIndex))
            (CallFunction|OnQueueUpdated)
            (return))))))
  (return))

(fn OnQueueUpdated
  (bind _expressionqueue (Variables|Default|GetExpressionQueue))
  (if (Utilities|Array|IsEmpty _expressionqueue)
    (CallFunction|ResetExpression)
    (else
      (CallFunction|SetExpression (Utilities|Array|Get(acopy) _expressionqueue (Utilities|Array|LastIndex _expressionqueue))))))

(fn RemoveExpression
  (params (Expression :type E_Expressions%20Enum :default "NewEnumerator4"))
  (bind _returnvalue (Utilities|Array|RemoveItem (Variables|Default|GetExpressionQueue) Expression))
  (if _returnvalue
    (CallFunction|OnQueueUpdated)))