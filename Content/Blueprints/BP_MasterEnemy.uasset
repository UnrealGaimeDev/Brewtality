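; Base enemy character that chases the teapot player after a spawn delay and destroys itself on contact, dealing damage.
; A stats component drives health, speed, damage and knockback, with health mirrored in material saturation.
; Hits flash materials and launch the enemy, enabling collision damage, while slows lower custom time dilation.
; Kills activate a pre-spawned breakable and drop luck-weighted sugar experience, plus card-gated health and ingredient pickups.
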(event OnComponentBeginOverlap(CapsuleComponent)
  (params (OverlappedComponent :type Primitive%20Component%20Object%20Reference) (OtherActor :type Actor%20Object%20Reference) (OtherComp :type Primitive%20Component%20Object%20Reference) (OtherBodyIndex :type Integer) (bFromSweep :type Boolean) (SweepResult :type Hit%20Result%20Structure%20%28by%20ref%29))
  (if (not (Variables|Default|GetDead?))
    (if (Variables|Default|GetInKnockback?)
      (Utilities|IsValid OtherActor
        (:Is%20Valid
          (CallFunction|OnKnockbackCollision OtherActor)))
      (elif (Utilities|Enum|NotEqual(Enum) (Variables|Default|GetState) "NewEnumerator0")
        (bind _asbp_teapot (Utilities|Casting|CastToBP_Teapot OtherActor))
        (bind _out_ (Default|CanReceiveDamage? _asbp_teapot (Utilities|Struct|MakeS_Damage 1e+01 "NewEnumerator1" self)))
        (if _out_
          (bind _value (Default|GetFinalValue (Variables|Default|GetEnemyStats) "damage"))
          (Default|ReceiveDamage _asbp_teapot (Utilities|Struct|MakeS_Damage _value "NewEnumerator1" self))
          (CallFunction|OnDeath false)
          (else
            (CallFunction|OnDeath false)))))))

(event OnComponentHit(CapsuleComponent)
  (params (HitComponent :type Primitive%20Component%20Object%20Reference) (OtherActor :type Actor%20Object%20Reference) (OtherComp :type Primitive%20Component%20Object%20Reference) (NormalImpulse :type Vector :default "0, 0, 0") (Hit :type Hit%20Result%20Structure%20%28by%20ref%29))
  (if (Variables|Default|GetInKnockback?)
    (CallFunction|OnKnockbackCollision OtherActor)))

(event Custom|OnDeath
  (params (ByKill? :type Boolean))
  (bind _breakableactor (Variables|Destruction|GetBreakableActor))
  (bind _breakableactor_2 (Variables|Destruction|GetBreakableActor))
  ;[0.15 0.15 0.15 0.5] Death
  (Variables|Default|SetDead? true)
  (if ByKill?
    (bind _location (CallFunction|GetExpLocation))
    (bind _output_get (Variables|Default|SetSpawnLoc _location))
    (CallFunction|TrySpawnHealthPickup _output_get)
    (CallFunction|TrySpawnIngredient _output_get)
    (CallFunction|ModifyExpQuantities)
    (bind _randomquantity (CallFunction|GenerateRandomExpQuantity))
    (if (Utilities|Enum|Equal(Enum) _randomquantity "NewEnumerator3")
      _
      (else
        (Game|SpawnActorfromClass "/Game/Blueprints/BP_Pickup_Sugar.BP_Pickup_Sugar_C" (Math|Transform|MakeTransform (Variables|Default|GetSpawnLoc)) "Undefined" "MultiplyWithRoot" 0 _randomquantity 0)))
    (Rendering|SetVisibility (Variables|Collision|GetCapsuleComponent) true true)
    (Utilities|IsValid _breakableactor
      (:Is%20Valid
        (Transformation|SetActorTransform (Variables|Destruction|GetBreakableActor) (Transformation|GetWorldTransform (Variables|Character|GetMesh)))
        (Default|ActivateBreakable _breakableactor))
      (:Is%20Not%20Valid
        _))
    (CallFunction|PlaySound "/Game/Audio/SFX/SC_EnemyDeath.SC_EnemyDeath" true (Transformation|GetWorldLocation (Variables|Character|GetMesh)))
    (bind _asbp_teapot_controller (Utilities|Casting|CastToBP_TeapotController (Game|GetPlayerController 0))
      (:then
        (Default|PlayForceFeedbackOnce _asbp_teapot_controller "/Game/Feedback/FF_Kill.FF_Kill"))
      (:CastFailed
        _))
    (Utilities|FlowControl|Delay 0.05)
    (Actor|DestroyActor)
    (else
      (Utilities|IsValid _breakableactor_2
        (:Is%20Valid
          (Actor|DestroyActor _breakableactor_2))
        (:Is%20Not%20Valid
          _))
      (Actor|DestroyActor))))

(event Custom|OnStatChanged
  (params (Stat :type String) (TotalValue :type Float%20%28double-precision%29))
  (switch string Stat
    (:health
      (bind _percentage (Default|GetPercentage (Variables|Default|GetEnemyStats) "health"))
      (for _array_element (Variables|Default|GetDynamicMaterials)
        (Rendering|Material|SetScalarParameterValue _array_element "Saturation" _percentage :!class /Script/Engine.MaterialInstanceDynamic)))
    (:speed
      (Variables|/Script/Engine.CharacterMovementComponent|SetMaxWalkSpeed (Variables|Character|GetCharacterMovement) TotalValue))))

(event Custom|OnKnockbackCollision
  (params (CollidedActor :type Actor%20Object%20Reference))
  (if (not (Variables|Default|GetTakenKnockbackDamage?))
    (if (Actor|ActorHasTag CollidedActor "damage_on_collision")
      (Variables|Default|SetTakenKnockbackDamage? true)
      (bind _teapot (CallFunction|GetTeapot))
      (bind (_out_ _damage) (Default|ShouldDealKnockbackDamage? _teapot))
      (if _out_
        (for _array_element (Utilities|Array|MakeArray CollidedActor self)
          (bind _out__2 (Class|IDamageable|CanReceiveDamage?(Message) _array_element (Utilities|Struct|MakeS_Damage _damage "NewEnumerator0" _teapot)))
          (if _out__2
            (Class|IDamageable|ReceiveDamage(Message) _array_element (Utilities|Struct|MakeS_Damage _damage "NewEnumerator0" _teapot))))))))

(event Custom|OnHit
  (params (DamageInfo :type S%20Damage%20Structure))
  (bind (_sourceactor _knockback) (Utilities|Struct|BreakS_Damage DamageInfo))
  (bind _enemystats (Variables|Default|GetEnemyStats))
  (CallFunction|FlashColor "(R=1.000000,G=0.132028,B=0.051229,A=1.000000)" 2e+01 0.2)
  (bind _value (Default|GetFinalValue _enemystats "knockback_resistance"))
  (bind _value_2 (Default|GetFinalValue _enemystats "knockback_factor"))
  (if (> (* _value_2 (- _knockback _value)) 0.0)
    (Variables|Default|SetInKnockback? true)
    (Components|Movement|StopMovementImmediately (Variables|Character|GetCharacterMovement))
    (Transformation|SetActorRotation (Math|Rotator|FindLookatRotation (CallFunction|RemoveZ (Transformation|GetActorLocation)) (CallFunction|RemoveZ (Transformation|GetActorLocation _sourceactor))))
    (Character|LaunchCharacter (* (* (Transformation|GetActorForwardVector) -1.0) (* _value_2 (- _knockback _value))) false false)
    (Utilities|FlowControl|RetriggerableDelay 0.2)
    (Variables|Default|SetInKnockback? false)
    (Variables|Default|SetTakenKnockbackDamage? false)))

(event Custom|FlashColor
  (params (Color :type Linear%20Color%20Structure :default "(R=1.000000,G=1.000000,B=1.000000,A=1.000000)") (Emissiveness :type Float%20%28double-precision%29) (Duration :type Float%20%28double-precision%29))
  (for _array_element (Variables|Default|GetDynamicMaterials)
    (Rendering|Material|SetVectorParameterValue _array_element "EmissiveColor" Color :!class /Script/Engine.MaterialInstanceDynamic)
    (Rendering|Material|SetScalarParameterValue _array_element "EmissiveStrength" Emissiveness :!class /Script/Engine.MaterialInstanceDynamic))
  (Utilities|FlowControl|Delay Duration)
  (for _array_element_2 (Variables|Default|GetDynamicMaterials)
    (Rendering|Material|SetVectorParameterValue :self _array_element_2 :ParameterName "EmissiveColor" :!class /Script/Engine.MaterialInstanceDynamic)
    (Rendering|Material|SetScalarParameterValue _array_element_2 "EmissiveStrength" 0.0 :!class /Script/Engine.MaterialInstanceDynamic)))

(event Custom|MoveToPlayer
  (AI|AIMoveTo self "0, 0, 0" (Game|Player|GetPlayerPawn 0) 5.0 false))

(event Custom|ApplySlowToEnemy
  (params (SlowStrength :type Float%20%28double-precision%29) (MinDilation :type Float%20%28double-precision%29) (Duration :type Float%20%28double-precision%29))
  ;[0.15 0.15 0.15 0.5] Slow
  (if (Variables|Default|GetSlowed?)
    _
    (else
      (CallFunction|OnSlowStart)))
  (Variables|Default|SetCustomTimeDilation (Math|Float|Max(Float) (- (Variables|Default|GetCustomTimeDilation) (/ SlowStrength 1e+02)) (Math|Float|Max(Float) MinDilation (CallFunction|GetMinDilation))))
  (Components|Timeline|SetPlayRate (Variables|Default|GetSlowTimeline) (/ 1.0 Duration))
  (Timeline|SlowTimeline PlayFromStart
    (:Finished
      (CallFunction|OnSlowEnd))))

(event Custom|OnSlowStart
  ;[0.15 0.15 0.15 0.5] Slow
  (Variables|Default|SetSlowed? true)
  (Default|AddEffect (Variables|Default|GetEffectBoxWidget) "NewEnumerator1")
  (bind _returnvalue (Utilities|Time|SetTimerbyFunctionName self "SlowTick" 1.0 true))
  (Variables|Default|SetSlowTimerHandle _returnvalue))

(event Custom|OnSlowEnd
  ;[0.15 0.15 0.15 0.5] Slow
  (Variables|Default|SetCustomTimeDilation 1.0)
  (Variables|Default|SetSlowed? false)
  (Default|RemoveEffect (Variables|Default|GetEffectBoxWidget) "NewEnumerator1")
  (Utilities|Time|ClearandInvalidateTimerbyHandle (Variables|Default|GetSlowTimerHandle)))

(event Custom|OnLifeBegin
  (Variables|Default|SetState "NewEnumerator1")
  (CallFunction|MovetoPlayer)
  (Utilities|Time|SetTimerbyEvent (delegate Custom|MoveToPlayer) 0.5 true))

(event Custom|OnLifeEnd
  (params (ByKill? :type Boolean) (ThroughKnockback? :type Boolean))
  (Variables|Default|SetState "NewEnumerator3")
  (if ThroughKnockback?
    (bind _teapot (CallFunction|GetTeapot))
    (Default|AddKnockbackKill (Variables|/Game/Blueprints/BP_Teapot.BP_Teapot_C|GetPlayerStatistics _teapot)))
  (CallFunction|OnDeath ByKill?))

(event EventBeginPlay
  (bind _enemystats (Variables|Default|GetEnemyStats))
  (Rendering|SetVisibility (Variables|Character|GetMesh) false true)
  (Utilities|Time|SetTimerbyFunctionName 0 "GroundLocationCheck" 0.35 true)
  (bind _aswbp_effect_box (Utilities|Casting|CastToWBP_EffectBox (UserInterface|GetUserWidgetObject (Variables|Default|GetEffectBox)))
    (:then
      (Variables|Default|SetEffectBoxWidget _aswbp_effect_box))
    (:CastFailed
      _))
  (CallFunction|GetDynamicMaterials)
  (EventDispatchers|BindEventtoOnStatValueChanged _enemystats (delegate Custom|OnStatChanged))
  (Default|InitializeValues _enemystats)
  (bind _returnvalue (Game|SpawnActorfromClass "/Game/Blueprints/BP_Breakable.BP_Breakable_C" (Math|Transform|MakeTransform "0, 0, 0" "0, 0, 0" (Transformation|GetWorldScale (Variables|Character|GetMesh))) "Undefined" "MultiplyWithRoot" 0 (Variables|Destruction|GetBreakableCollection) 0))
  (Variables|Destruction|SetBreakableActor _returnvalue)
  (Default|ResetValuetoMax (Variables|Default|GetEnemyStats) "health")
  (Utilities|FlowControl|Delay (Variables|Default|GetSpawnDelay))
  (Components|DestroyComponent (Variables|Default|GetSpawnDecal))
  (Rendering|SetVisibility (Variables|Character|GetMesh) true true)
  (CallFunction|OnLifeBegin))

(event EventDamage
  (params (Damage :type S%20Damage%20Structure))
  (bind (_amount _sourcetype _sourceactor _knockback _critical_ _type) (Utilities|Struct|BreakS_Damage Damage))
  (bind _enemystats (Variables|Default|GetEnemyStats))
  (if (not (Variables|Default|GetDead?))
    (if (and (Utilities|Enum|Equal(Enum) _sourcetype "NewEnumerator0") (Utilities|Enum|Equal(Enum) _type "NewEnumerator0"))
      (Math|Integer|IncrementInt (Variables|Default|GetProjectilesTaken)
        (:%20%20
          _)))
    (bind _value (Default|GetFinalValue _enemystats "health"))
    (Variables|Default|SetPreviousHealth _value)
    (Default|ModifyBaseValue _enemystats "health" (* _amount -1.0))
    (bind _value_2 (Default|GetFinalValue (Variables|Default|GetEnemyStats) "health"))
    (Variables|Default|SetNewHealth _value_2)
    (CallFunction|PlaySound (.Value (Utilities|Map|Find (Variables|Feedback|GetDamagedSounds) _type)) true (Transformation|GetWorldLocation (Variables|Character|GetMesh)))
    (Game|SpawnActorfromClass "/Game/Blueprints/BP_DamageNumber.BP_DamageNumber_C" (Math|Transform|MakeTransform (+ (Transformation|GetWorldLocation (Variables|Character|GetMesh)) (Variables|Feedback|GetDamageNumberOffset))) "AlwaysSpawn" "MultiplyWithRoot" 0 Damage 0)
    (bind _structout (Utilities|Struct|SetmembersinS_Damage Damage (- (Variables|Default|GetPreviousHealth) (Variables|Default|GetNewHealth))))
    (if (<= (Variables|Default|GetNewHealth) 0.01)
      (Utilities|FlowControl|Sequence
        (:then_0
          (Variables|Default|SetDead? true)
          (Class|IDamageable|OnDamageDealt(Message) _sourceactor self _structout true))
        (:then_1
          (CallFunction|OnLifeEnd true (Utilities|Enum|Equal(Enum) _type "NewEnumerator4"))))
      (else
        (CallFunction|OnHit Damage)
        (Class|IDamageable|OnDamageDealt(Message) _sourceactor self _structout false)))))

(event EventSetDotActor
  (params (Dot :type BP%20Dot%20Damage%20Object%20Reference))
  (Variables|Default|SetAppliedDot Dot))

(fn ConstructionScript)

(fn GenerateRandomExpQuantity
  (bind _experiencedropweights (Variables|Reward|GetExperienceDropWeights))
  (bind _keys (Utilities|Map|Keys _experiencedropweights))
  (LocalVariables|SetlocalKeys _keys)
  (bind _values (Utilities|Map|Values _experiencedropweights))
  (LocalVariables|SetlocalWeights _values)
  (for _array_element (LocalVariables|GetlocalWeights)
    (LocalVariables|SetlocalWeightsSum (+ _array_element (LocalVariables|GetlocalWeightsSum))))
  (LocalVariables|SetlocalRandom (Math|Random|RandomFloatinRange 0.0 (LocalVariables|GetlocalWeightsSum)))
  (bind (_array_element_2 _array_index) (Utilities|Array|ForEachLoopwithBreak (LocalVariables|GetlocalKeys) :!label _label)
    (:LoopBody
      (if (< (LocalVariables|GetlocalRandom) (+ (LocalVariables|GetlocalPassedSum) (Utilities|Array|Get(acopy) (LocalVariables|GetlocalWeights) _array_index)))
        (LocalVariables|SetlocalFound _array_element_2)
        (goto _label Break)
        (else
          (LocalVariables|SetlocalPassedSum (+ (LocalVariables|GetlocalPassedSum) (Utilities|Array|Get(acopy) (LocalVariables|GetlocalWeights) _array_index))))))
    (:Completed
      (return (LocalVariables|GetlocalFound)))))

(fn ModifyExpQuantities
  (bind _teapot (CallFunction|GetTeapot))
  (bind _value (Default|GetFinalValue (Variables|/Game/Blueprints/BP_Teapot.BP_Teapot_C|GetCharacterStats _teapot) "luck"))
  (LocalVariables|SetlocalLuck _value)
  (bind _keys (Utilities|Map|Keys (Variables|Reward|GetExperienceDropWeights)))
  (for _array_element _keys
    (bind _output_get (LocalVariables|SetlocalPrevious (.Value (Utilities|Map|Find (Variables|Reward|GetExperienceDropWeights) _array_element))))
    (if (!= _output_get 0.0)
      (bind _output_get_2 (LocalVariables|SetlocalPrevious (Math|Float|SelectFloat (Math|Float|Max(Float) (- (LocalVariables|GetlocalPrevious) (LocalVariables|GetlocalLuck)) 0.0) (Math|Float|Max(Float) (+ (LocalVariables|GetlocalPrevious) (LocalVariables|GetlocalLuck)) 0.0) (Utilities|Enum|Equal(Enum) _array_element "NewEnumerator3"))))
      (Utilities|Map|Add (Variables|Reward|GetExperienceDropWeights) _array_element _output_get_2)))
  (return))

(fn GetDynamicMaterials
  (for _array_element (Actor|GetComponentsByClass "/Script/Engine.SkeletalMeshComponent")
    (for (_array_element_2 _array_index) (Rendering|Material|GetMaterials _array_element)
      (bind _returnvalue (Rendering|Material|CreateDynamicMaterialInstance _array_element _array_index _array_element_2 "None" :!class /Script/Engine.PrimitiveComponent))
      (Utilities|Array|Add (Variables|Default|GetDynamicMaterials) _returnvalue))))

(fn GroundLocationCheck
  (if (AI|Components|NavMovement|IsFalling (Variables|Character|GetCharacterMovement))
    _
    (else
      (bind _ground (CallFunction|FindGroundLocation self))
      (Variables|Default|SetLastGroundLocation _ground)))
  (return))

(fn GetExpLocation
  (if (AI|Components|NavMovement|IsFalling (Variables|Character|GetCharacterMovement))
    (return (Variables|Default|GetLastGroundLocation))
    (else
      (bind _ground (CallFunction|FindGroundLocation self))
      (return _ground))))

(fn SlowTick
  (bind _teapot (CallFunction|GetTeapot))
  (Default|AddSlowDuration (Variables|/Game/Blueprints/BP_Teapot.BP_Teapot_C|GetPlayerStatistics _teapot) 1.0))

(fn GetTeapot
  (Utilities|IsValid (Variables|Default|GetTeapotRef)
    (:Is%20Valid
      _)
    (:Is%20Not%20Valid
      (bind _asbp_teapot (Utilities|Casting|CastToBP_Teapot (Game|Player|GetPlayerPawn 0)))
      (Variables|Default|SetTeapotRef _asbp_teapot)))
  (return (Variables|Default|GetTeapotRef)))

(fn GetMinDilation
  (return (.Value (Utilities|Map|Find (Variables|Default|GetMinTimeDilationsByType) (Variables|Type|GetEnemyType)))))

(fn TrySpawnHealthPickup
  (params (SpawnLocation :type Vector))
  (bind _healthdropmaxoffset (Variables|Default|GetHealthDropMaxOffset))
  (bind _healthdropmaxoffset_2 (Variables|Default|GetHealthDropMaxOffset))
  (if (< (Math|Random|RandomIntegerinRange 0 99) (Variables|Reward|GetHealthDropChance))
    (bind _instance (CallFunction|GetGameInstance))
    (bind _out (Default|HasCard? _instance "health_drop"))
    (if _out
      (Game|SpawnActorfromClass "/Game/Blueprints/BP_Pickup_Health.BP_Pickup_Health_C" (Math|Transform|MakeTransform (+ SpawnLocation (Math|Vector|MakeVector (Math|Random|RandomFloatinRange (* _healthdropmaxoffset_2 -1.0) _healthdropmaxoffset_2) (Math|Random|RandomFloatinRange (* _healthdropmaxoffset -1.0) _healthdropmaxoffset) 0.0))) "Undefined" "MultiplyWithRoot" 0 0)
      (return)
      (else
        (return)))
    (else
      (return))))

(fn GetGameInstance
  (Utilities|IsValid (Variables|Default|GetGameInstance)
    (:Is%20Valid
      _)
    (:Is%20Not%20Valid
      (bind _asgi_brewtality (Utilities|Casting|CastToGI_Brewtality (Game|GetGameInstance)))
      (Variables|Default|SetGameInstance _asgi_brewtality)))
  (return (Variables|Default|GetGameInstance)))

(fn TrySpawnIngredient
  (params (SpawnLocation :type Vector))
  (bind _healthdropmaxoffset (Variables|Default|GetHealthDropMaxOffset))
  (bind _healthdropmaxoffset_2 (Variables|Default|GetHealthDropMaxOffset))
  (switch Utilities|FlowControl|Switch|SwitchonE_EnemyTypes (Variables|Type|GetEnemyType)
    (:NewEnumerator0
      (return))
    (:NewEnumerator1
      _)
    (:NewEnumerator2
      _)
    (:NewEnumerator3
      (return)))
  (if (< (Math|Random|RandomIntegerinRange 0 99) (Variables|Reward|GetIngredientDropChance))
    (bind _instance (CallFunction|GetGameInstance))
    (bind _out (Default|HasCard? _instance "ingredient_drop"))
    (if _out
      (bind _teapot (CallFunction|GetTeapot))
      (Game|SpawnActorfromClass "/Game/Blueprints/BP_Pickup_Ingredient.BP_Pickup_Ingredient_C" (Math|Transform|MakeTransform (+ SpawnLocation (Math|Vector|MakeVector (Math|Random|RandomFloatinRange (* _healthdropmaxoffset_2 -1.0) _healthdropmaxoffset_2) (Math|Random|RandomFloatinRange (* _healthdropmaxoffset -1.0) _healthdropmaxoffset) 0.0))) "Undefined" "MultiplyWithRoot" 0 (.OutItem (Utilities|Array|Random (Variables|/Game/Blueprints/BpC_Ingredients.BpC_Ingredients_C|GetAvailableIngredients (Variables|/Game/Blueprints/BP_Teapot.BP_Teapot_C|GetIngredients _teapot)))) 0)
      (return)
      (else
        (return)))
    (else
      (return))))

(fn CanReceiveDamage?
  (params (Damage :type S%20Damage%20Structure))
  (return (and (Utilities|Enum|NotEqual(Enum) (.SourceType (Utilities|Struct|BreakS_Damage Damage)) "NewEnumerator1") (not (Variables|Default|GetDead?)))))

(fn GetDotActor
  (return (Variables|Default|GetAppliedDot)))