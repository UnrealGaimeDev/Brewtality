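; BP_LeftBorder is a moving border that trails the player along the Y axis and limits how far the follow camera can go.
; A looping timer moves it to the larger of its current Y and the player pawn's Y plus an offset, so it only ever advances toward positive Y.
; Each update also sets the YLimit of BP_FollowCamera to the border's Y plus a camera offset.
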(event Custom|UpdatePosition
  (bind _returnvalue (Transformation|GetActorLocation))
  (bind (_x _y _z) (Math|Vector|BreakVector _returnvalue))
  (Transformation|SetActorLocation (Math|Vector|MakeVector _x (Math|Float|Max(Float) _y (+ (.Y (Math|Vector|BreakVector (Transformation|GetActorLocation (Game|Player|GetPlayerPawn 0)))) (Variables|Default|GetYOffset))) _z) false false)
  (bind _returnvalue_2 (Actor|GetActorOfClass "/Game/Blueprints/BP_FollowCamera.BP_FollowCamera_C"))
  (Utilities|IsValid _returnvalue_2
    (:Is%20Valid
      (Variables|/Game/Blueprints/BP_FollowCamera.BP_FollowCamera_C|SetYLimit _returnvalue_2 (+ _y (Variables|Default|GetCameraYOffset))))))

(event EventBeginPlay
  (Utilities|Time|SetTimerbyEvent (delegate Custom|UpdatePosition) 0.2 true))

(fn ConstructionScript)