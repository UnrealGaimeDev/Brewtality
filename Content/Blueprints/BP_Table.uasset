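; BP_Table is a tiled table that scrolls forward along Y as a BP_Teapot reaches its end.
; Construction lays startup tiles as instanced meshes and sizes EndBox, which sits on the last tile.
; Teapot overlap removes two rear tiles and appends two ahead, moving EndBox and recentering the scaled NavMesh volume.
; After a short delay, a console command rebuilds navigation and the DoOnce guard resets.
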(event OnComponentBeginOverlap(EndBox)
  (params (OverlappedComponent :type Primitive%20Component%20Object%20Reference) (OtherActor :type Actor%20Object%20Reference) (OtherComp :type Primitive%20Component%20Object%20Reference) (OtherBodyIndex :type Integer) (bFromSweep :type Boolean) (SweepResult :type Hit%20Result%20Structure%20%28by%20ref%29))
  (Utilities|Casting|CastToBP_Teapot OtherActor)
  (Utilities|FlowControl|DoOnce false :!label _label
    (:Completed
      (CallFunction|RemoveTiles 2)
      (CallFunction|AddTiles 2)
      (Utilities|FlowControl|Delay 0.2)
      (Development|ExecuteConsoleCommand "RebuildNavigation" 0)
      (goto _label Reset))))

(event EventBeginPlay)

(event Collision|EventActorBeginOverlap
  (params (OtherActor :type Actor%20Object%20Reference)))

(event EventTick
  (params (DeltaSeconds :type Float%20%28single-precision%29)))

(fn ConstructionScript
  (bind _tilewidth (Variables|Generation|GetTileWidth))
  (bind _returnvalue (/ _tilewidth 2.0))
  (bind _output_get (Variables|Default|SetFirstTileLocation (Transformation|GetWorldLocation (Variables|Default|GetDefaultSceneRoot))))
  (Variables|Default|SetLastTileLocation (- _output_get (Math|Vector|MakeVector 0.0 (Variables|Generation|GetTileWidth) 0.0)))
  (Components|Box|SetBoxExtent (Variables|Default|GetEndBox) (Math|Vector|MakeVector _returnvalue _returnvalue 1e+02) false)
  (CallFunction|AddTiles (Variables|Generation|GetStartupTiles)))

(fn AddTiles
  (params (Amount :type Integer))
  (bind _navmesh (Variables|Default|GetNavMesh))
  (Variables|Default|SetNumberOfTiles (+ (Variables|Default|GetNumberOfTiles) Amount))
  (for _index (range 0 (- Amount 1))
    (bind _output_get (Variables|Default|SetLastTileLocation (+ (Variables|Default|GetLastTileLocation) (Math|Vector|MakeVector 0.0 (Variables|Generation|GetTileWidth) 0.0))))
    (Components|InstancedStaticMesh|AddInstance (Variables|Default|GetInstancedStaticMesh) (Math|Transform|MakeTransform _output_get) true))
  (Transformation|SetWorldLocation (Variables|Default|GetEndBox) (Variables|Default|GetLastTileLocation) false false)
  (Transformation|SetWorldScale3D (Variables|/Script/Engine.Brush|GetBrushComponent _navmesh) (Math|Vector|MakeVector 1.0 (Math|Conversions|ToFloat(Integer) (Variables|Default|GetNumberOfTiles)) 1.0))
  (Transformation|SetActorLocation _navmesh (CallFunction|GetCenterLocation) false false))

(fn GetCenterLocation
  (return (/ (+ (Variables|Default|GetLastTileLocation) (Variables|Default|GetFirstTileLocation)) 2.0)))

(fn RemoveTiles
  (params (Amount :type Integer))
  (for _index (range 0 (- Amount 1))
    (Utilities|Array|Add (LocalVariables|GetlocalIndices) _index))
  (Class|InstancedStaticMeshComponent|RemoveInstances (Variables|Default|GetInstancedStaticMesh) (LocalVariables|GetlocalIndices))
  (Variables|Default|SetNumberOfTiles (- (Variables|Default|GetNumberOfTiles) Amount))
  (Variables|Default|SetFirstTileLocation (+ (Variables|Default|GetFirstTileLocation) (Math|Vector|MakeVector 0.0 (* Amount (Variables|Generation|GetTileWidth)) 0.0))))