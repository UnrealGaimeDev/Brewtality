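; Floating damage number actor that shows the amount of one hit through its DamageWidget component, then removes itself.
; On BeginPlay it writes the truncated DamageInfo amount into the WBP_DamageNumber text, tinted with the crit or default color.
; It then reveals the widget, plays its animation and destroys itself when the widget's animation-finished event fires.
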(event Custom|OnWidgetAnimEnd
  (Actor|DestroyActor))

(event EventBeginPlay
  (bind _damageinfo (Variables|Default|GetDamageInfo))
  (bind (_amount _critical_) (Utilities|Struct|BreakS_Damage _damageinfo))
  (bind _aswbp_damage_number (Utilities|Casting|CastToWBP_DamageNumber (UserInterface|GetUserWidgetObject (Variables|Default|GetDamageWidget))))
  (bind _output_get (Variables|Default|SetNumberWidgetRef _aswbp_damage_number))
  (Rendering|Components|TextRender|SetText (Variables|/Game/UserInterface/WBP_DamageNumber.WBP_DamageNumber_C|GetNumberText _output_get) (Utilities|Text|ToText(Integer) (Math|Float|Truncate _amount) false false))
  (Appearance|SetColorandOpacity (Variables|/Game/UserInterface/WBP_DamageNumber.WBP_DamageNumber_C|GetNumberText _output_get) (Utilities|Struct|MakeSlateColor (Math|Color|SelectColor (Variables|Appearance|GetCritColor) (Variables|Appearance|GetDefaultColor) _critical_) "UseColor_Specified") :!class /Script/UMG.TextBlock)
  (Rendering|SetVisibility (Variables|Default|GetDamageWidget) true false)
  (EventDispatchers|BindEventtoOnAnimFinished (Variables|Default|GetNumberWidgetRef) (delegate Custom|OnWidgetAnimEnd))
  (Default|PlayAnim (Variables|Default|GetNumberWidgetRef)))

(fn ConstructionScript)