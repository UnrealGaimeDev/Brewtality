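; Stats component that stores named stats with base, min, max and modifiers, and exposes functions to query, modify and reset them.
; Final values add flat modifiers to the base, scale by summed percentage modifiers, then clamp to range.
; Edits write structs back to the Stats map, then UpdateFinalValue recalculates, broadcasts OnStatValueChanged and refreshes that stat's widget.
; Widgets are generated in StatDisplayOrder for stats in the DisplayStats set.
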(event EventBeginPlay)

(event EventTick
  (params (DeltaSeconds :type Float%20%28single-precision%29)))

(fn CalculateFinalValue
  (params (Stat :type String))
  (LocalVariables|SetlocalStat Stat)
  (LocalVariables|SetlocalStatInfo (.Values (Utilities|Struct|BreakS_StatInfo (.Value (Utilities|Map|Find (Variables|Default|GetStats) (LocalVariables|GetlocalStat))))))
  (LocalVariables|SetlocalBase (.BaseValue (Utilities|Struct|BreakS_StatValues (LocalVariables|GetlocalStatInfo))))
  (LocalVariables|SetlocalMin (.MinValue (Utilities|Struct|BreakS_StatValues (LocalVariables|GetlocalStatInfo))))
  (LocalVariables|SetlocalMax (.MaxValue (Utilities|Struct|BreakS_StatValues (LocalVariables|GetlocalStatInfo))))
  (for _array_element (.Modifiers (Utilities|Struct|BreakS_StatValues (LocalVariables|GetlocalStatInfo)))
    (LocalVariables|SetlocalFlat (+ (LocalVariables|GetlocalFlat) (.FlatModifier (Utilities|Struct|BreakS_StatModifier _array_element))))
    (LocalVariables|SetlocalPerc (+ (LocalVariables|GetlocalPerc) (.PercentageModifier (Utilities|Struct|BreakS_StatModifier _array_element)))))
  (bind _output_get (LocalVariables|SetlocalFinal (Math|Float|Clamp(Float) (* (+ (LocalVariables|GetlocalBase) (LocalVariables|GetlocalFlat)) (+ 1.0 (LocalVariables|GetlocalPerc))) (LocalVariables|GetlocalMin) (LocalVariables|GetlocalMax))))
  (return _output_get))

(fn UpdateFinalValue
  (params (Stat :type String))
  (LocalVariables|SetlocalStatString Stat)
  (if (.ReturnValue (Utilities|Map|Find (Variables|Default|GetStats) (LocalVariables|GetlocalStatString)))
    (LocalVariables|SetlocalStatInfo (.Value (Utilities|Map|Find (Variables|Default|GetStats) (LocalVariables|GetlocalStatString))))
    (bind _finalvalue (CallFunction|CalculateFinalValue (LocalVariables|GetlocalStatString)))
    (LocalVariables|SetlocalFinal _finalvalue)
    (bind _output_get (LocalVariables|SetlocalValues (.Values (Utilities|Struct|BreakS_StatInfo (LocalVariables|GetlocalStatInfo)))))
    (bind _structout (Utilities|Struct|SetmembersinS_StatValues _output_get (LocalVariables|GetlocalFinal)))
    (bind _structout_2 (Utilities|Struct|SetmembersinS_StatInfo (LocalVariables|GetlocalStatInfo) _structout))
    (Utilities|Map|Add (Variables|Default|GetStats) (LocalVariables|GetlocalStatString) _structout_2)
    (Default|CallOnStatValueChanged (LocalVariables|GetlocalStatString) (LocalVariables|GetlocalFinal))
    (Utilities|IsValid (.Value (Utilities|Map|Find (Variables|Default|GetStatWidgets) (LocalVariables|GetlocalStatString)))
      (:Is%20Valid
        (Default|UpdateValueDisplay (.Value (Utilities|Map|Find (Variables|Default|GetStatWidgets) (LocalVariables|GetlocalStatString))) (LocalVariables|GetlocalValues)))
      (:Is%20Not%20Valid
        _))
    (return true)
    (else
      (return false))))

(fn InitializeValues
  (bind _keys (Utilities|Map|Keys (Variables|Default|GetStats)))
  (for _array_element _keys
    (CallFunction|UpdateFinalValue _array_element))
  (return))

(fn GetFinalValue
  (params (Stat :type String))
  (bind _stats (Variables|Default|GetStats))
  (bind (_value _returnvalue) (Utilities|Map|Find _stats Stat))
  (if _returnvalue
    (return true (Utilities|Struct|BreakS_StatValues (.Values (Utilities|Struct|BreakS_StatInfo _value))))
    (else
      (return false 0.0))))

(fn GetMaxValue
  (params (Stat :type String))
  (bind _stats (Variables|Default|GetStats))
  (bind (_value _returnvalue) (Utilities|Map|Find _stats Stat))
  (if _returnvalue
    (return true (Utilities|Struct|BreakS_StatValues (.Values (Utilities|Struct|BreakS_StatInfo _value))))
    (else
      (return false 0.0))))

(fn ModifyBaseValue
  (params (Stat :type String) (Modifier :type Float%20%28double-precision%29))
  (LocalVariables|SetlocalStat Stat)
  (LocalVariables|SetlocalMod Modifier)
  (if (.ReturnValue (Utilities|Map|Find (Variables|Default|GetStats) (LocalVariables|GetlocalStat)))
    (LocalVariables|SetlocalStatInfo (.Value (Utilities|Map|Find (Variables|Default|GetStats) (LocalVariables|GetlocalStat))))
    (LocalVariables|SetlocalValues (.Values (Utilities|Struct|BreakS_StatInfo (LocalVariables|GetlocalStatInfo))))
    (LocalVariables|SetlocalPreviousBase (.BaseValue (Utilities|Struct|BreakS_StatValues (LocalVariables|GetlocalValues))))
    (LocalVariables|SetlocalNewBase (Math|Float|Clamp(Float) (+ (.BaseValue (Utilities|Struct|BreakS_StatValues (LocalVariables|GetlocalValues))) (LocalVariables|GetlocalMod)) (.MinValue (Utilities|Struct|BreakS_StatValues (LocalVariables|GetlocalValues))) (.MaxValue (Utilities|Struct|BreakS_StatValues (LocalVariables|GetlocalValues)))))
    (LocalVariables|SetlocalRemainder (- (LocalVariables|GetlocalMod) (- (LocalVariables|GetlocalNewBase) (LocalVariables|GetlocalPreviousBase))))
    (bind _structout (Utilities|Struct|SetmembersinS_StatValues (LocalVariables|GetlocalValues) (LocalVariables|GetlocalNewBase)))
    (bind _structout_2 (Utilities|Struct|SetmembersinS_StatInfo (LocalVariables|GetlocalStatInfo) _structout))
    (Utilities|Map|Add (Variables|Default|GetStats) (LocalVariables|GetlocalStat) _structout_2)
    (bind _success_ (CallFunction|UpdateFinalValue (LocalVariables|GetlocalStat)))
    (return _success_ (LocalVariables|GetlocalRemainder))
    (else
      (return false 0.0))))

(fn GetPercentage
  (params (Stat :type String))
  (bind _stats (Variables|Default|GetStats))
  (bind _value (Utilities|Map|Find _stats Stat))
  (bind _values (Utilities|Struct|BreakS_StatInfo _value))
  (bind (_minvalue _maxvalue _totalvalue) (Utilities|Struct|BreakS_StatValues _values))
  (return (/ (- _totalvalue _minvalue) (- _maxvalue _minvalue))))

(fn ResetValuetoMin
  (params (Stat :type String))
  (LocalVariables|SetlocalNam Stat)
  (if (.ReturnValue (Utilities|Map|Find (Variables|Default|GetStats) (LocalVariables|GetlocalNam)))
    (LocalVariables|SetlocalStatInfo (.Value (Utilities|Map|Find (Variables|Default|GetStats) (LocalVariables|GetlocalNam))))
    (LocalVariables|SetlocalValues (.Values (Utilities|Struct|BreakS_StatInfo (LocalVariables|GetlocalStatInfo))))
    (bind _structout (Utilities|Struct|SetmembersinS_StatValues (LocalVariables|GetlocalValues) (Utilities|Struct|BreakS_StatValues (LocalVariables|GetlocalValues)) (Utilities|Array|MakeArray)))
    (bind _structout_2 (Utilities|Struct|SetmembersinS_StatInfo (LocalVariables|GetlocalStatInfo) _structout))
    (Utilities|Map|Add (Variables|Default|GetStats) (LocalVariables|GetlocalNam) _structout_2)
    (bind _success_ (CallFunction|UpdateFinalValue (LocalVariables|GetlocalNam)))
    (return _success_)
    (else
      (return false))))

(fn ModifyMaxValue
  (params (Stat :type String) (Modifier :type Float%20%28double-precision%29))
  (LocalVariables|SetlocalStat Stat)
  (LocalVariables|SetlocalMod Modifier)
  (if (.ReturnValue (Utilities|Map|Find (Variables|Default|GetStats) (LocalVariables|GetlocalStat)))
    (LocalVariables|SetlocalStatInfo (.Value (Utilities|Map|Find (Variables|Default|GetStats) (LocalVariables|GetlocalStat))))
    (LocalVariables|SetlocalValues (.Values (Utilities|Struct|BreakS_StatInfo (LocalVariables|GetlocalStatInfo))))
    (bind _structout (Utilities|Struct|SetmembersinS_StatValues (LocalVariables|GetlocalValues) (+ (Utilities|Struct|BreakS_StatValues (LocalVariables|GetlocalValues)) (LocalVariables|GetlocalMod))))
    (bind _structout_2 (Utilities|Struct|SetmembersinS_StatInfo (LocalVariables|GetlocalStatInfo) _structout))
    (Utilities|Map|Add (Variables|Default|GetStats) (LocalVariables|GetlocalStat) _structout_2)
    (bind _success_ (CallFunction|UpdateFinalValue (LocalVariables|GetlocalStat)))
    (return _success_)
    (else
      (return false))))

(fn AddStatModifier
  (params (Stat :type String) (Modifier :type S%20Stat%20Modifier%20Structure))
  (LocalVariables|SetlocalStat Stat)
  (LocalVariables|SetlocalModifier Modifier)
  (if (.ReturnValue (Utilities|Map|Find (Variables|Default|GetStats) (LocalVariables|GetlocalStat)))
    (LocalVariables|SetlocalStatInfo (.Value (Utilities|Map|Find (Variables|Default|GetStats) (LocalVariables|GetlocalStat))))
    (LocalVariables|SetlocalValues (.Values (Utilities|Struct|BreakS_StatInfo (LocalVariables|GetlocalStatInfo))))
    (LocalVariables|SetlocalModifiers (Utilities|Struct|BreakS_StatValues (LocalVariables|GetlocalValues)))
    (Utilities|Array|Add (LocalVariables|GetlocalModifiers) (LocalVariables|GetlocalModifier))
    (bind _structout (Utilities|Struct|SetmembersinS_StatValues (LocalVariables|GetlocalValues) (LocalVariables|GetlocalModifiers)))
    (bind _structout_2 (Utilities|Struct|SetmembersinS_StatInfo (LocalVariables|GetlocalStatInfo) _structout))
    (Utilities|Map|Add (Variables|Default|GetStats) (LocalVariables|GetlocalStat) _structout_2)
    (bind _success_ (CallFunction|UpdateFinalValue (LocalVariables|GetlocalStat)))
    (return _success_)
    (else
      (return false))))

(fn ResetValuetoMax
  (params (Stat :type String))
  (LocalVariables|SetlocalNam Stat)
  (if (.ReturnValue (Utilities|Map|Find (Variables|Default|GetStats) (LocalVariables|GetlocalNam)))
    (LocalVariables|SetlocalStatInfo (.Value (Utilities|Map|Find (Variables|Default|GetStats) (LocalVariables|GetlocalNam))))
    (LocalVariables|SetlocalValues (.Values (Utilities|Struct|BreakS_StatInfo (LocalVariables|GetlocalStatInfo))))
    (bind _structout (Utilities|Struct|SetmembersinS_StatValues (LocalVariables|GetlocalValues) (Utilities|Struct|BreakS_StatValues (LocalVariables|GetlocalValues)) (Utilities|Array|MakeArray)))
    (bind _structout_2 (Utilities|Struct|SetmembersinS_StatInfo (LocalVariables|GetlocalStatInfo) _structout))
    (Utilities|Map|Add (Variables|Default|GetStats) (LocalVariables|GetlocalNam) _structout_2)
    (bind _success_ (CallFunction|UpdateFinalValue (LocalVariables|GetlocalNam)))
    (return _success_)
    (else
      (return false))))

(fn GenerateStatWidgets
  (params (MainWidget :type WBP%20Main%20Object%20Reference))
  (bind _output_get (Variables|Default|SetMainWidget MainWidget))
  (Widget|Panel|ClearChildren (Variables|/Game/UserInterface/WBP_Main.WBP_Main_C|GetAttributesBox _output_get))
  (Utilities|Map|Clear (Variables|Default|GetStatWidgets))
  (for _array_element (Variables|Default|GetStatDisplayOrder)
    (if (Utilities|Set|Contains (Variables|Default|GetDisplayStats) _array_element)
      (bind _widget (Default|AddStatDisplay (Variables|Default|GetMainWidget) (.Value (Utilities|Map|Find (Variables|Default|GetStats) _array_element))))
      (Utilities|Map|Add (Variables|Default|GetStatWidgets) _array_element _widget))))

(fn AddDisplayStats
  (params (Stats :type Array%20of%20Strings))
  (bind _mainwidget (Variables|Default|GetMainWidget))
  (Utilities|Set|AddItems (Variables|Default|GetDisplayStats) Stats)
  (Utilities|IsValid _mainwidget
    (:Is%20Valid
      (CallFunction|GenerateStatWidgets _mainwidget))
    (:Is%20Not%20Valid
      _))
  (return))