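; Enemy spawner actor that endlessly spawns enemies at random reachable navigation points within a radius, escalating over time.
; A looping delay from BeginPlay shrinks by a multiplier after each spawn, down to a minimum interval.
; A spawn counter picks BP_MasterEnemy or periodically BP_EliteEnemy, and each elite lowers the count until the next, down to a minimum.
; The construction script sizes the SpawnRadius sphere to match the radius.
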(event EventBeginPlay
  (bind _spawnradius (Variables|Default|GetSpawnRadius))
  (bind _radius (Variables|SpawnBehaviour|GetRadius))
  (bind _returnvalue (Transformation|GetWorldLocation _spawnradius))
  (bind _randomlocation (AI|Navigation|GetRandomReachablePointinRadius _returnvalue _radius 0 0))
  (bind _returnvalue_2 (Math|Transform|MakeTransform _randomlocation))
  (Utilities|FlowControl|Delay (Variables|SpawnBehaviour|GetInitialSpawnDelay) :!label _label)
  (if (== (Math|Integer|%(Integer) (Variables|Default|GetSpawnedEnemies) (Variables|SpawnBehaviour|GetEnemiesUntilElite)) 0)
    (Game|SpawnActorfromClass "/Game/Blueprints/BP_EliteEnemy.BP_EliteEnemy_C" _returnvalue_2 "Undefined" "MultiplyWithRoot" 0 0)
    (Variables|SpawnBehaviour|SetEnemiesUntilElite (Math|Integer|Max(Integer) (- (Variables|SpawnBehaviour|GetEnemiesUntilElite) 1) (Variables|SpawnBehaviour|GetMinEnemiesUntilElite)))
    (Variables|Default|SetSpawnedEnemies 1)
    (else
      (Game|SpawnActorfromClass "/Game/Blueprints/BP_MasterEnemy.BP_MasterEnemy_C" _returnvalue_2 "Undefined" "MultiplyWithRoot" 0 0)
      (Math|Integer|IncrementInt (Variables|Default|GetSpawnedEnemies)
        (:%20%20
          _))))
  (Variables|SpawnBehaviour|SetInitialSpawnDelay (Math|Float|Max(Float) (* (Variables|SpawnBehaviour|GetInitialSpawnDelay) (Variables|SpawnBehaviour|GetDelayMultiplier)) (Variables|SpawnBehaviour|GetMinInterval)))
  (goto _label))

(fn ConstructionScript
  (Components|Sphere|SetSphereRadius (Variables|Default|GetSpawnRadius) (Variables|SpawnBehaviour|GetRadius) true))