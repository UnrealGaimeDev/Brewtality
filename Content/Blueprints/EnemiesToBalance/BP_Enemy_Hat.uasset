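; Hat enemy that periodically unleashes special attacks: a shockwave AoE, a radial card volley or summoned Thimbles.
; A self-repeating tick picks a random attack, briefly pauses movement and waits a random interval, until death.
; Attack values come from EnemyStats, with shockwave and cards spawned relative to player height.
; Per-attack cooldowns are tracked, but GetAvailableAttack removes every key from the cooldown set, so they don't restrict selection.
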(event Custom|SpawnThimbles
  (bind _enemystats (Variables|Default|GetEnemyStats))
  (bind _value (Default|GetFinalValue _enemystats "thimble_spawn_radius"))
  (Variables|Default|SetSpawnRadius _value)
  (bind _value_2 (Default|GetFinalValue _enemystats "thimble_spawn_number"))
  (for _index (range 1 (Math|Float|Truncate _value_2))
    (if (.ReturnValue (AI|Navigation|GetRandomReachablePointinRadius (Transformation|GetActorLocation) (Variables|Default|GetSpawnRadius) 0 0))
      (Game|SpawnActorfromClass "/Game/Blueprints/EnemiesToBalance/BP_Enemy_Thimble.BP_Enemy_Thimble_C" (Math|Transform|MakeTransform (.RandomLocation (AI|Navigation|GetRandomReachablePointinRadius (Transformation|GetActorLocation) (Variables|Default|GetSpawnRadius) 0 0))) "AdjustIfPossibleButDontSpawnIfColliding" "MultiplyWithRoot" 0 0))))

(event Custom|FireCards
  (bind _cardsymbols (Variables|Default|GetCardSymbols))
  (bind _enemystats (Variables|Default|GetEnemyStats))
  (bind _value (Default|GetFinalValue _enemystats "card_number_low"))
  (bind _value_2 (Default|GetFinalValue _enemystats "card_number_high"))
  (Variables|Default|SetNumberOfCards (Math|Integer|SelectInt (Math|Float|Truncate _value_2) (Math|Float|Truncate _value) (Math|Random|RandomBool)))
  (Variables|Default|SetDegrees (/ 3.6e+02 (Math|Conversions|ToFloat(Integer) (Variables|Default|GetNumberOfCards))))
  (bind _value_3 (Default|GetFinalValue _enemystats "card_damage"))
  (bind _value_4 (Default|GetFinalValue _enemystats "card_range"))
  (Variables|Default|SetCardRange _value_4)
  (bind _value_5 (Default|GetFinalValue _enemystats "card_speed"))
  (Variables|Default|SetCardSpeed _value_5)
  (Utilities|Struct|SetmembersinS_Damage (Variables|Default|GetCardDamage) _value_3 "NewEnumerator1" self)
  (for _index (range 0 (- (Variables|Default|GetNumberOfCards) 1))
    (Game|SpawnActorfromClass "/Game/Blueprints/BP_CardProjectile.BP_CardProjectile_C" (Math|Transform|MakeTransform (Math|Vector|MakeVector (.X (Math|Vector|BreakVector (+ (Transformation|GetActorLocation) (* (Math|Vector|GetForwardVector (Math|Rotator|MakeRotator 0.0 0.0 (* _index (Variables|Default|GetDegrees)))) 2e+02)))) (.Y (Math|Vector|BreakVector (+ (Transformation|GetActorLocation) (* (Math|Vector|GetForwardVector (Math|Rotator|MakeRotator 0.0 0.0 (* _index (Variables|Default|GetDegrees)))) 2e+02)))) (- (.Z (Math|Vector|BreakVector (Transformation|GetActorLocation (Game|Player|GetPlayerPawn 0)))) 3e+01)) (Math|Rotator|MakeRotator 0.0 0.0 (* _index (Variables|Default|GetDegrees)))) "Undefined" "MultiplyWithRoot" 0 (Utilities|Array|Get(acopy) _cardsymbols (Math|Integer|%(Integer) _index (Utilities|Array|Length _cardsymbols))) (Variables|Default|GetCardRange) (Variables|Default|GetCardDamage) (Variables|Default|GetCardSpeed) 0)))

(event Custom|PerformAttack
  (params (Attack :type E_BossAttacks%20Enum :default "NewEnumerator0"))
  (bind _attacksoncooldown (Variables|Default|GetAttacksOnCooldown))
  (if (not (Utilities|Set|Contains _attacksoncooldown Attack))
    (Utilities|Set|Add _attacksoncooldown Attack)
    (switch Utilities|FlowControl|Switch|SwitchonE_BossAttacks Attack
      (:NewEnumerator0
        (CallFunction|PerformShockwave)
        (bind _cooldown (CallFunction|GetAttackCooldown Attack))
        (Utilities|FlowControl|Delay _cooldown)
        (Utilities|Set|Remove (Variables|Default|GetAttacksOnCooldown) Attack))
      (:NewEnumerator1
        (CallFunction|FireCards)
        (bind _cooldown_2 (CallFunction|GetAttackCooldown Attack))
        (Utilities|FlowControl|Delay _cooldown_2)
        (Utilities|Set|Remove (Variables|Default|GetAttacksOnCooldown) Attack))
      (:NewEnumerator2
        (CallFunction|SpawnThimbles)
        (bind _cooldown_3 (CallFunction|GetAttackCooldown Attack))
        (Utilities|FlowControl|Delay _cooldown_3)
        (Utilities|Set|Remove (Variables|Default|GetAttacksOnCooldown) Attack)))))

(event Custom|PerformShockwave
  (bind _returnvalue (Transformation|GetActorLocation))
  (bind (_x _y) (Math|Vector|BreakVector _returnvalue))
  (bind _returnvalue_2 (Game|SpawnActorfromClass "/Game/Blueprints/BP_AoE_HatShockwave.BP_AoE_HatShockwave_C" (Math|Transform|MakeTransform (Math|Vector|MakeVector _x _y (- (.Z (Math|Vector|BreakVector (Transformation|GetActorLocation (Game|Player|GetPlayerPawn 0)))) 3e+01))) "AlwaysSpawn" "MultiplyWithRoot" 0 0))
  (bind _value (Default|GetFinalValue (Variables|Default|GetEnemyStats) "shockwave_damage"))
  (Default|TriggerAoE _returnvalue_2 (Utilities|Struct|MakeS_Damage _value "NewEnumerator1" self 0.0 false "NewEnumerator2") 5e+03 0.0 0.0))

(event Custom|SpecialAttackTick
  (if (Variables|Default|GetKeepAttacking?)
    (bind (_success_ _attack) (CallFunction|GetAvailableAttack))
    (if _success_
      (CallFunction|PauseMovement)
      (CallFunction|PerformAttack _attack)
      (Utilities|FlowControl|Delay 0.4)
      (CallFunction|ResumeMovement))
    (Utilities|FlowControl|Delay (Math|Random|RandomFloatinRange (Variables|Behaviour|GetMinAttackPause) (Variables|Behaviour|GetMaxAttackPause)))
    (CallFunction|SpecialAttackTick)))

(event EventBeginPlay
  (|CallParentFunction)
  (Utilities|FlowControl|Delay 2.0)
  (CallFunction|SpecialAttackTick))

(event EventOnDeath
  (params (ByKill? :type Boolean))
  (Variables|Default|SetKeepAttacking? false)
  (|CallParentFunction ByKill?))

(fn ConstructionScript
  (|CallParentFunction))

(fn GetAttackCooldown
  (params (Attack :type E_BossAttacks%20Enum%20%28by%20ref%29 :default "NewEnumerator0"))
  (return (.Value (Utilities|Map|Find (Variables|Behaviour|GetAttackCooldowns) Attack))))

(fn GetAvailableAttack
  (bind _keys (Utilities|Map|Keys (Variables|Behaviour|GetAttackCooldowns)))
  (bind _output_get (LocalVariables|SetlocalAttacks _keys))
  (Utilities|Set|RemoveItems (Variables|Default|GetAttacksOnCooldown) _output_get)
  (if (Utilities|Array|IsEmpty (LocalVariables|GetlocalAttacks))
    (return false "NewEnumerator0")
    (else
      (return true (.OutItem (Utilities|Array|Random (LocalVariables|GetlocalAttacks)))))))