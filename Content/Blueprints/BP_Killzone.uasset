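; BP_Killzone is a box-shaped volume that deals effectively lethal damage to damageable actors that enter it.
; The construction script sizes the Collision box from the Width and Height variables, with Width used for both horizontal axes.
; On begin overlap, it checks the other actor for I_Damageable and sends a huge critical damage message through that interface, naming itself as the source.
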(event OnComponentBeginOverlap(Collision)
  (params (OverlappedComponent :type Primitive%20Component%20Object%20Reference) (OtherActor :type Actor%20Object%20Reference) (OtherComp :type Primitive%20Component%20Object%20Reference) (OtherBodyIndex :type Integer) (bFromSweep :type Boolean) (SweepResult :type Hit%20Result%20Structure%20%28by%20ref%29))
  (if (Utilities|DoesObjectImplementInterface OtherActor "/Game/Blueprints/Interfaces/I_Damageable.I_Damageable_C")
    (Class|IDamageable|ReceiveDamage(Message) OtherActor (Utilities|Struct|MakeS_Damage 9999.0 "NewEnumerator2" self 0.0 true "NewEnumerator4"))))

(event EventBeginPlay)

(event Collision|EventActorBeginOverlap
  (params (OtherActor :type Actor%20Object%20Reference)))

(event EventTick
  (params (DeltaSeconds :type Float%20%28single-precision%29)))

(fn ConstructionScript
  (Components|Box|SetBoxExtent (Variables|Default|GetCollision) (Math|Vector|MakeVector (Variables|Dimensions|GetWidth) (Variables|Dimensions|GetWidth) (Variables|Dimensions|GetHeight)) true))