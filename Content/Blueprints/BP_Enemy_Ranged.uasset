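; Ranged enemy child Blueprint that fires salves of BP_EnemyProjectile at the player.
; A looping timer polls horizontal range and WorldStatic line of sight, then pauses movement and starts a fire-rate timer.
; The salve ends on duration, lost shot or death, then movement resumes during a cooldown.
; Shots spawn near player height and fly level with random yaw spread, with all combat tuning read from EnemyStats.
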(event Custom|ShootCheck
  (if (and (not (Variables|Default|GetShooting?)) (not (Variables|Default|GetAttackOnCooldown?)))
    (bind _out_ (CallFunction|CanShoot?))
    (if _out_
      (CallFunction|StartSalve))))

(event Custom|StartSalve
  (if (not (Variables|Default|GetShooting?))
    (Variables|Default|SetShooting? true)
    (CallFunction|PauseMovement)
    (Variables|Default|SetSalveDuration 0.0)
    (CallFunction|FireatPlayer)
    (bind _value (Default|GetFinalValue (Variables|Default|GetEnemyStats) "fire_rate"))
    (bind _output_get (Variables|Default|SetFireInterval (/ 1.0 _value)))
    (bind _returnvalue (Utilities|Time|SetTimerbyEvent (delegate Custom|SalveTick) _output_get true))
    (Variables|Default|SetSalveTimer _returnvalue)))

(event Custom|SalveTick
  (bind _out_ (CallFunction|CanShoot?))
  (if _out_
    (CallFunction|FireatPlayer)
    (bind _output_get (Variables|Default|SetSalveDuration (+ (Variables|Default|GetSalveDuration) (Variables|Default|GetFireInterval))))
    (bind _value (Default|GetFinalValue (Variables|Default|GetEnemyStats) "salve_duration"))
    (if (>= _output_get _value)
      (CallFunction|StopSalve))
    (else
      (CallFunction|StopSalve))))

(event Custom|StopSalve
  (if (Variables|Default|GetShooting?)
    (Variables|Default|SetShooting? false)
    (Variables|Default|SetAttackOnCooldown? true)
    (Utilities|Time|ClearandInvalidateTimerbyHandle (Variables|Default|GetSalveTimer))
    (CallFunction|ResumeMovement)
    (bind _value (Default|GetFinalValue (Variables|Default|GetEnemyStats) "attack_cooldown"))
    (Utilities|FlowControl|Delay _value)
    (Variables|Default|SetAttackOnCooldown? false)))

(event EventBeginPlay
  (|CallParentFunction)
  (Utilities|Time|SetTimerbyEvent (delegate Custom|ShootCheck) 0.15 true))

(event EventDamage
  (params (Damage :type S%20Damage%20Structure))
  (|CallParentFunction Damage))

(event EventSetDotActor
  (params (Dot :type BP%20Dot%20Damage%20Object%20Reference))
  (|CallParentFunction Dot))

(event EventOnDamageDealt
  (params (HurtActor :type Actor%20Object%20Reference) (DamageInfo :type S%20Damage%20Structure) (Lethal? :type Boolean))
  (|CallParentFunction HurtActor DamageInfo Lethal?))

(event EventOnDeath
  (params (ByKill? :type Boolean))
  (CallFunction|StopSalve)
  (|CallParentFunction ByKill?))

(fn ConstructionScript
  (|CallParentFunction))

(fn FireatPlayer
  (bind _returnvalue (Game|Player|GetPlayerPawn 0))
  (bind _returnvalue_2 (Transformation|GetActorLocation))
  (bind _projectilepoint (Variables|Default|GetProjectilePoint))
  (bind _enemystats (Variables|Default|GetEnemyStats))
  (bind _returnvalue_3 (Transformation|GetActorLocation _returnvalue))
  (bind _returnvalue_4 (Transformation|GetWorldLocation _projectilepoint))
  (bind _returnvalue_5 (Math|Rotator|FindLookatRotation _returnvalue_2 _returnvalue_3))
  (bind (_x _y) (Math|Vector|BreakVector _returnvalue_4))
  (bind _value (Default|GetFinalValue _enemystats "projectile_range"))
  (bind _value_2 (Default|GetFinalValue _enemystats "projectile_speed"))
  (bind _value_3 (Default|GetFinalValue _enemystats "damage"))
  (bind _value_4 (Default|GetFinalValue _enemystats "aim_offset"))
  (Transformation|SetActorRotation _returnvalue_5)
  (CallFunction|SpawnProjectile (Math|Transform|MakeTransform (Math|Vector|MakeVector _x _y (- (.Z (Math|Vector|BreakVector _returnvalue_3)) 3e+01)) (Math|Rotator|MakeRotator 0.0 0.0 (+ (.Yaw (Math|Rotator|BreakRotator _returnvalue_5)) (Math|Random|RandomFloatinRange (* _value_4 -1.0) _value_4)))) _value (Utilities|Struct|MakeS_Damage _value_3 "NewEnumerator1" self) _value_2))

(fn HasLineOfSight?
  (bind _returnvalue (Collision|LineTraceForObjects (Transformation|GetActorLocation (Game|Player|GetPlayerPawn 0)) (Transformation|GetWorldLocation (Variables|Default|GetProjectilePoint)) (Utilities|Array|MakeArray "ObjectTypeQuery1") false (Utilities|Array|MakeArray (Game|Player|GetPlayerPawn 0)) "None"))
  (return (not _returnvalue)))

(fn InRange?
  (bind _value (Default|GetFinalValue (Variables|Default|GetEnemyStats) "attack_range"))
  (return (>= _value (Math|Vector|Distance(Vector) (CallFunction|RemoveZ (Transformation|GetActorLocation (Game|Player|GetPlayerPawn 0))) (CallFunction|RemoveZ (Transformation|GetActorLocation self))))))

(fn CanShoot?
  (bind _out_ (CallFunction|InRange?))
  (if _out_
    (bind _out__2 (CallFunction|HasLineOfSight?))
    (if _out__2
      (return true)
      (else
        (return false)))
    (else
      (return false))))

(fn CanReceiveDamage?
  (params (Damage :type S%20Damage%20Structure))
  (bind _out_ (|CallParentFunction Damage))
  (return _out_))

(fn GetDotActor
  (bind _dot (|CallParentFunction))
  (return _dot))

(fn SpawnProjectile
  (params (Transform :type Transform) (TravelDistance :type Float%20%28double-precision%29) (Damage :type S%20Damage%20Structure) (Speed :type Float%20%28double-precision%29))
  (Game|SpawnActorfromClass "/Game/Blueprints/BP_EnemyProjectile.BP_EnemyProjectile_C" Transform "Undefined" "MultiplyWithRoot" 0 TravelDistance Damage Speed 0))