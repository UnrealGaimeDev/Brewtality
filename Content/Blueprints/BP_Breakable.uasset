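; BP_Breakable is an actor that plays a physics-driven break effect from an assigned geometry collection, then removes itself.
; BeginPlay creates a dynamic material and hides the collection, destroying the actor if none is assigned.
; ActivateBreakable reveals the collection, enables physics and applies a strong impulse away from the player with an upward bias.
; After a delay, a timeline drives the material's MaskOpacity to dissolve the pieces before destroying the actor.
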(event Custom|Destruct
  (Physics|AddImpulse (Variables|Default|GetGeometryCollection) (* (Math|Vector|Normalize (+ (CallFunction|RemoveZ (- (Transformation|GetActorLocation) (Transformation|GetActorLocation (Game|Player|GetPlayerPawn 0)))) "0.000000,0.000000,0.700000")) 4e+05) "None" false))

(event Custom|Dissolve
  (bind _opacity (Timeline|DissolveTimeline PlayFromStart)
    (:Update
      (Rendering|Material|SetScalarParameterValue (Variables|Default|GetDynamicMat) "MaskOpacity" _opacity :!class /Script/Engine.MaterialInstanceDynamic))
    (:Finished
      (Actor|DestroyActor))))

(event Custom|ActivateBreakable
  (bind _geometrycollection (Variables|Default|GetGeometryCollection))
  (Physics|SetSimulatePhysics _geometrycollection true)
  (CallFunction|Destruct)
  (Rendering|SetVisibility _geometrycollection true false)
  (Utilities|FlowControl|Delay (Variables|Default|GetTimeBeforeRemoval))
  (Utilities|IsValid (Variables|Default|GetDynamicMat)
    (:Is%20Valid
      (CallFunction|Dissolve))
    (:Is%20Not%20Valid
      (Actor|DestroyActor))))

(event EventBeginPlay
  (bind _geometrycollection (Variables|Default|GetGeometryCollection))
  (bind _breakablecollection (Variables|Default|GetBreakableCollection))
  (bind _returnvalue (Rendering|Material|CreateDynamicMaterialInstance _geometrycollection 0 (Rendering|Material|GetMaterial _geometrycollection 0) "None" :!class /Script/Engine.PrimitiveComponent))
  (Variables|Default|SetDynamicMat _returnvalue)
  (Rendering|Material|SetScalarParameterValue (Variables|Default|GetDynamicMat) "Saturation" 0.0 :!class /Script/Engine.MaterialInstanceDynamic)
  (Utilities|IsValid _breakablecollection
    (:Is%20Valid
      (Class|GeometryCollectionComponent|SetRestCollection (Variables|Default|GetGeometryCollection) _breakablecollection false)
      (Rendering|SetVisibility (Variables|Default|GetGeometryCollection) false true))
    (:Is%20Not%20Valid
      (Actor|DestroyActor))))

(fn ConstructionScript)