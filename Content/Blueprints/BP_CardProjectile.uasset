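; BP_CardProjectile is a card projectile actor whose mesh displays one of the four suits, chosen by CardSymbol.
; The construction script creates a dynamic material instance from the mesh's first material and sets its UvX and UvY parameters per suit, selecting a quadrant of what appears to be a shared texture atlas.
; The event graph holds only disabled stub events, so this Blueprint's graphs add no runtime logic.
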(event EventBeginPlay
  (|CallParentFunction) ; This node is disabled and will not be called.\nDrag off pins to build functionality.
)

(event Collision|EventActorBeginOverlap
  (params (OtherActor :type Actor%20Object%20Reference)))

(event EventTick
  (params (DeltaSeconds :type Float%20%28single-precision%29)))

(fn ConstructionScript
  (bind _mesh (Variables|Character|GetMesh))
  (|CallParentFunction)
  (bind _returnvalue (Rendering|Material|CreateDynamicMaterialInstance _mesh 0 (Rendering|Material|GetMaterial _mesh 0) "None" :!class /Script/Engine.PrimitiveComponent))
  (Rendering|Material|SetScalarParameterValue _returnvalue "UvX" (Utilities|Select :Index (Variables|Default|GetCardSymbol) :NewEnumerator5 0.0 :NewEnumerator0 0.4808 :NewEnumerator1 0.0 :NewEnumerator2 0.0 :NewEnumerator3 0.4808) :!class /Script/Engine.MaterialInstanceDynamic)
  (Rendering|Material|SetScalarParameterValue _returnvalue "UvY" (Utilities|Select :Index (Variables|Default|GetCardSymbol) :NewEnumerator5 0.0 :NewEnumerator0 0.0 :NewEnumerator1 0.0 :NewEnumerator2 0.5 :NewEnumerator3 0.5) :!class /Script/Engine.MaterialInstanceDynamic))