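; Fire trail segment actor with an Area volume that tracks enemies standing in it and thins out crowded segments.
; When another trail overlaps Area within a small fixed distance, it removes that one from the referenced Teapot's trail and destroys it.
; GetOverlappingEnemies returns the BP_MasterEnemy actors inside Area; the segment itself applies no effect to them.
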(event OnComponentBeginOverlap(Area)
  (params (OverlappedComponent :type Primitive%20Component%20Object%20Reference) (OtherActor :type Actor%20Object%20Reference) (OtherComp :type Primitive%20Component%20Object%20Reference) (OtherBodyIndex :type Integer) (bFromSweep :type Boolean) (SweepResult :type Hit%20Result%20Structure%20%28by%20ref%29))
  (bind _asbp_firetrail (Utilities|Casting|CastToBP_Firetrail OtherActor))
  (if (< (Math|Vector|Distance(Vector) (Transformation|GetActorLocation _asbp_firetrail) (Transformation|GetActorLocation)) 5e+01)
    (Default|RemoveTrail (Variables|Default|GetTeapot) _asbp_firetrail)
    (Actor|DestroyActor _asbp_firetrail)))

(event EventBeginPlay)

(event Collision|EventActorBeginOverlap
  (params (OtherActor :type Actor%20Object%20Reference)))

(event EventTick
  (params (DeltaSeconds :type Float%20%28single-precision%29)))

(fn ConstructionScript)

(fn GetOverlappingEnemies
  (return (Collision|GetOverlappingActors (Variables|Default|GetArea) "/Game/Blueprints/BP_MasterEnemy.BP_MasterEnemy_C" :!class /Script/Engine.PrimitiveComponent)))