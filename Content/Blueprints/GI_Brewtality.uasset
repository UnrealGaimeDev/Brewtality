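; Game instance for Brewtality that owns card-collection progression, its save slot and the cards menu.
; Init caps the frame rate at 60, then loads the save or resets to startup values.
; Card progress is checked against DT_Cards goals, and reaching one activates the card.
; Activation feeds the heart_queen meta-card and uncovers deck-grid neighbours: the whole column vertically, one card to each side.
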(event Custom|CreateCardsMenu
  (bind _returnvalue (UserInterface|CreateWidget "/Game/UserInterface/WBP_CardsMenu.WBP_CardsMenu_C" (Game|GetPlayerController 0) self))
  (bind _output_get (Variables|Default|SetCardsMenuRef _returnvalue))
  (Default|GenerateCards _output_get (Variables|Default|GetCardDeck) (Variables|Default|GetSuitDisplayOrder))
  (UserInterface|Viewport|AddtoViewport (Variables|Default|GetCardsMenuRef) 20))

(event Custom|CloseCardsMenu
  (Widget|RemovefromParent (Variables|Default|GetCardsMenuRef))
  (Variables|Default|SetCardsMenuRef 0))

(event Custom|OnProgressUpdated
  (params (Card :type Name))
  (if (not (Utilities|Set|Contains (Variables|Default|GetActivatedCards) Card))
    (bind (_current _max) (CallFunction|GetCardProgress Card))
    (if (>= _current _max)
      (CallFunction|ActivateCard Card))))

(event Custom|ActivateCard
  (params (Card :type Name%20%28by%20ref%29))
  (bind _activatedcards (Variables|Default|GetActivatedCards))
  (Utilities|Set|Add _activatedcards Card)
  (Utilities|Set|Add (Variables|Default|GetDiscoveredCards) Card)
  (CallFunction|AddCardProgress "heart_queen" (Math|Conversions|ToFloat(Integer) (Utilities|Set|Length _activatedcards)) "NewEnumerator1")
  (bind _cardstouncover (CallFunction|GetCardstoUncover Card))
  (for _array_element _cardstouncover
    (Utilities|Set|Add (Variables|Default|GetDiscoveredCards) _array_element)))

(event EventInit
  (bind _returnvalue (Settings|GetGameUserSettings))
  (Class|GameUserSettings|SetFrameRateLimit _returnvalue 6e+01)
  (Class|GameUserSettings|ApplySettings _returnvalue true)
  (if (Variables|SaveLoad|GetLoadGameOnStart?)
    (bind _success_ (CallFunction|LoadGame))
    (if _success_
      (Variables|SaveLoad|SetHasLoadedGame? true)
      (else
        (CallFunction|ResetValues :!label _label)))
    (else
      (goto _label))))

(fn GetCardDeck
  (return (Variables|Default|GetCardDeck)))

(fn GetNeighborinDirection
  (params (Position :type S%20Card%20Position%20Structure) (Direction :type E_Directions%20Enum :default "NewEnumerator4"))
  (bind (_suit _face) (Utilities|Struct|BreakS_CardPosition Position))
  (bind _suitdisplayorder (Variables|Default|GetSuitDisplayOrder))
  (bind _carddeck (Variables|Default|GetCardDeck))
  (bind _returnvalue (Utilities|Array|FindItem _suitdisplayorder _suit))
  (bind _value (Utilities|Map|Find _carddeck _suit))
  (bind _faces (Utilities|Struct|BreakS_CardSuit _value))
  (if (Utilities|Enum|Equal(Enum) Direction "NewEnumerator4")
    _
    (else
      (switch Utilities|FlowControl|Switch|SwitchonE_Directions Direction
        (:NewEnumerator4
          _)
        (:NewEnumerator0
          (if (>= _returnvalue 1)
            (return true (Utilities|Struct|MakeS_CardPosition (Utilities|Array|Get(acopy) (Variables|Default|GetSuitDisplayOrder) (- _returnvalue 1)) _face))
            (else
              _)))
        (:NewEnumerator1
          (bind _keys (Utilities|Map|Keys _faces))
          (if (< (Utilities|Array|FindItem _keys _face) (Utilities|Array|LastIndex _keys))
            (return true (Utilities|Struct|MakeS_CardPosition _suit (Utilities|Array|Get(acopy) _keys (+ (Utilities|Array|FindItem _keys _face) 1))))
            (else
              (return false ""))))
        (:NewEnumerator2
          (if (< _returnvalue (Utilities|Array|LastIndex _suitdisplayorder))
            (return true (Utilities|Struct|MakeS_CardPosition (Utilities|Array|Get(acopy) (Variables|Default|GetSuitDisplayOrder) (+ _returnvalue 1)) _face))
            (else
              _)))
        (:NewEnumerator3
          (bind _keys_2 (Utilities|Map|Keys _faces))
          (if (> (Utilities|Array|FindItem _keys_2 _face) 0)
            (return true (Utilities|Struct|MakeS_CardPosition _suit (Utilities|Array|Get(acopy) _keys_2 (- (Utilities|Array|FindItem _keys_2 _face) 1))))
            (else
              (return false "")))))))
  (return false ""))

(fn GetCardProgress
  (params (Card :type Name))
  (bind _cardprogress (Variables|Default|GetCardProgress))
  (bind (_value _returnvalue) (Utilities|Map|Find _cardprogress Card))
  (bind _returnvalue_2 (Utilities|GetDataTableRow "/Game/Blueprints/DataTables/DT_Cards.DT_Cards" Card)
    (:then
      (LocalVariables|SetlocalMax (Utilities|Struct|BreakS_Card _returnvalue_2))
      (LocalVariables|SetlocalCur (Math|Float|SelectFloat _value 0.0 _returnvalue))
      (return (LocalVariables|GetlocalCur) (LocalVariables|GetlocalMax) (Math|Float|Min(Float) (/ (LocalVariables|GetlocalCur) (LocalVariables|GetlocalMax)) 1.0)))
    (:RowNotFound
      (return -1.0 -1.0 -1.0))))

(fn GetCardState
  (params (Card :type Name))
  (if (Utilities|Set|Contains (Variables|Default|GetActivatedCards) Card)
    (return "NewEnumerator2")
    (elif (Utilities|Set|Contains (Variables|Default|GetDiscoveredCards) Card)
      (return "NewEnumerator1")
      (else
        (return "NewEnumerator0")))))

(fn AddCardProgress
  (params (Card :type Name) (Amount :type Float%20%28double-precision%29) (Mode :type E_ProgressModes%20Enum :default "NewEnumerator0"))
  (bind _cardprogress (Variables|Default|GetCardProgress))
  (bind (_value _returnvalue) (Utilities|Map|Find _cardprogress Card))
  (if _returnvalue
    (LocalVariables|SetlocalPrevious _value)
    (switch Utilities|FlowControl|Switch|SwitchonE_ProgressModes Mode
      (:NewEnumerator0
        (Utilities|Map|Add (Variables|Default|GetCardProgress) Card (+ (LocalVariables|GetlocalPrevious) Amount)))
      (:NewEnumerator1
        (if (< (LocalVariables|GetlocalPrevious) Amount)
          (Utilities|Map|Add (Variables|Default|GetCardProgress) Card Amount)
          (else
            (return)))))
    (CallFunction|OnProgressUpdated Card)
    (else
      (Utilities|Map|Add _cardprogress Card Amount)
      (CallFunction|OnProgressUpdated Card))))

(fn TryAddMaxedStats
  (params (Stats :type Array%20of%20Strings))
  (for _array_element Stats
    (Utilities|Set|Add (Variables|Default|GetMaxedStats) _array_element))
  (CallFunction|AddCardProgress "heat_shield" (Math|Conversions|ToFloat(Integer) (Utilities|Set|Length (Variables|Default|GetMaxedStats))) "NewEnumerator1"))

(fn SaveGame
  (bind _savegame (CallFunction|GetSaveGame))
  (Variables|/Game/Blueprints/SaveGame_Brewtality.SaveGame_Brewtality_C|SetSavedCardProgress _savegame (Variables|Default|GetCardProgress))
  (Variables|/Game/Blueprints/SaveGame_Brewtality.SaveGame_Brewtality_C|SetSavedDiscoveredCards _savegame (Variables|Default|GetDiscoveredCards))
  (Variables|/Game/Blueprints/SaveGame_Brewtality.SaveGame_Brewtality_C|SetSavedActivatedCards _savegame (Variables|Default|GetActivatedCards))
  (Variables|/Game/Blueprints/SaveGame_Brewtality.SaveGame_Brewtality_C|SetSavedMaxedStats _savegame (Variables|Default|GetMaxedStats))
  (SaveGame|SaveGametoSlot _savegame (Variables|SaveLoad|GetSaveSlot))
  (Variables|SaveLoad|SetHasSaved? true))

(fn GetSaveGame
  (Utilities|IsValid (Variables|SaveLoad|GetSaveGameRef)
    (:Is%20Valid
      _)
    (:Is%20Not%20Valid
      (bind _returnvalue (SaveGame|CreateSaveGameObject "/Game/Blueprints/SaveGame_Brewtality.SaveGame_Brewtality_C"))
      (Variables|SaveLoad|SetSaveGameRef _returnvalue)))
  (return (Variables|SaveLoad|GetSaveGameRef)))

(fn LoadGame
  (bind _returnvalue (SaveGame|LoadGamefromSlot (Variables|SaveLoad|GetSaveSlot)))
  (Utilities|IsValid _returnvalue
    (:Is%20Valid
      (bind _assave_game_brewtality (Utilities|Casting|CastToSaveGame_Brewtality _returnvalue)
        (:then
          (bind _output_get (Variables|SaveLoad|SetSaveGameRef _assave_game_brewtality))
          (Variables|Default|SetCardProgress (Variables|/Game/Blueprints/SaveGame_Brewtality.SaveGame_Brewtality_C|GetSavedCardProgress _output_get))
          (Variables|Default|SetDiscoveredCards (Variables|/Game/Blueprints/SaveGame_Brewtality.SaveGame_Brewtality_C|GetSavedDiscoveredCards _output_get))
          (Variables|Default|SetActivatedCards (Variables|/Game/Blueprints/SaveGame_Brewtality.SaveGame_Brewtality_C|GetSavedActivatedCards _output_get))
          (Variables|Default|SetMaxedStats (Variables|/Game/Blueprints/SaveGame_Brewtality.SaveGame_Brewtality_C|GetSavedMaxedStats _output_get))
          (return true))
        (:CastFailed
          _)))
    (:Is%20Not%20Valid
      _))
  (return false))

(fn DeleteSaveGame
  (SaveGame|DeleteGameinSlot (Variables|SaveLoad|GetSaveSlot))
  (Utilities|IsValid (Variables|SaveLoad|GetSaveGameRef)
    (:Is%20Valid
      (Variables|SaveLoad|SetSaveGameRef 0)
      (Variables|SaveLoad|SetHasSaved? false))
    (:Is%20Not%20Valid
      _))
  (CallFunction|ResetValues))

(fn ResetValues
  (Variables|Default|SetCardProgress (Utilities|Map|MakeMap))
  (Variables|Default|SetDiscoveredCards (Variables|Default|GetStartupDiscoveredCards))
  (Variables|Default|SetActivatedCards (Variables|Default|GetStartupActivatedCards))
  (Variables|Default|SetMaxedStats (Utilities|Set|MakeSet)))

(fn GetCardbyPosition
  (params (Position :type S%20Card%20Position%20Structure))
  (bind _output_get (LocalVariables|SetlocalPosition Position))
  (bind _deck (CallFunction|GetCardDeck))
  (if (.ReturnValue (Utilities|Map|Find _deck (.Suit (Utilities|Struct|BreakS_CardPosition _output_get))))
    (if (.ReturnValue (Utilities|Map|Find (Utilities|Struct|BreakS_CardSuit (.Value (Utilities|Map|Find _deck (.Suit (Utilities|Struct|BreakS_CardPosition _output_get))))) (.Face (Utilities|Struct|BreakS_CardPosition _output_get))))
      (return true (.Value (Utilities|Map|Find (Utilities|Struct|BreakS_CardSuit (.Value (Utilities|Map|Find _deck (.Suit (Utilities|Struct|BreakS_CardPosition _output_get))))) (.Face (Utilities|Struct|BreakS_CardPosition _output_get)))))
      (else
        _)))
  (return false "None"))

(fn FindCardPosition
  (params (Card :type Name))
  (LocalVariables|SetlocalCard Card)
  (bind (_keypin _valuepin) (Utilities|Map|ForEachLoop(Map) (Variables|Default|GetCardDeck) :!label _label)
    (:then
      (LocalVariables|SetlocalSuit _keypin)
      (bind (_keypin_2 _valuepin_2) (Utilities|Map|ForEachLoop(Map) (Utilities|Struct|BreakS_CardSuit _valuepin) :!label _label_2)
        (:then
          (LocalVariables|SetlocalFace _keypin_2)
          (if (== _valuepin_2 (LocalVariables|GetlocalCard))
            (Utilities|FlowControl|Sequence
              (:then_0
                (goto _label_2 BreakPin))
              (:then_1
                (goto _label BreakPin)))))))
    (:CompletedPin
      (return (Utilities|Struct|MakeS_CardPosition (LocalVariables|GetlocalSuit) (LocalVariables|GetlocalFace))))))

(fn GetCardstoUncover
  (params (ActivatedCard :type Name))
  (bind _position (CallFunction|FindCardPosition ActivatedCard))
  (LocalVariables|SetlocalPos _position)
  (bind _enumvalue (|ForEachE_Directions)
    (:LoopBody
      (switch Utilities|FlowControl|Switch|SwitchonE_Directions _enumvalue
        (:NewEnumerator0
          _)
        (:NewEnumerator1
          _)
        (:NewEnumerator2
          _)
        (:NewEnumerator3
          _))
      (bind _cards (CallFunction|GetCardsinDirection (LocalVariables|GetlocalPos) _enumvalue (or (Utilities|Enum|Equal(Enum) _enumvalue "NewEnumerator0") (Utilities|Enum|Equal(Enum) _enumvalue "NewEnumerator2"))))
      (for _array_element _cards
        (Utilities|Array|Add (LocalVariables|GetCardsToUncover) _array_element)))
    (:then
      (return (LocalVariables|GetCardsToUncover)))))

(fn GetCardsinDirection
  (params (Position :type S%20Card%20Position%20Structure) (Direction :type E_Directions%20Enum :default "NewEnumerator4") (KeepGoing? :type Boolean))
  (LocalVariables|SetlocalKeep KeepGoing?)
  (LocalVariables|SetlocalPos Position)
  (LocalVariables|SetlocalDir Direction)
  (bind (_success_ _neighborpos) (CallFunction|GetNeighborinDirection (LocalVariables|GetlocalPos) (LocalVariables|GetlocalDir) :!label _label))
  (if _success_
    (bind (_success__2 _name) (CallFunction|GetCardbyPosition _neighborpos))
    (if _success__2
      (Utilities|Array|Add (LocalVariables|GetlocalCards) _name)
      (if (LocalVariables|GetlocalKeep)
        (LocalVariables|SetlocalPos _neighborpos)
        (goto _label)
        (else
          _))))
  (return (LocalVariables|GetlocalCards)))

(fn HasCard?
  (params (Card :type Name))
  (return (Utilities|Set|Contains (Variables|Default|GetActivatedCards) Card)))